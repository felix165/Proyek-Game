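; Inventory system Blueprint that currently handles look-at detection for interaction; its add and remove inventory functions are empty stubs.
; Every tick, it sphere-traces forward from the player character up to InteractionRange, ignoring its owner.
; When the hit actor changes, it stores it as LookAtActor, calls LookAtMessage on it and prints the result.
; A miss clears LookAtActor.
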(event `self.ReceiveTick`
  (params (DeltaSeconds :type "Float (single-precision)"))
  (`self.interactionTrace`))

(fn `addToInventory`)

(fn `interactionTrace`
  (bind _returnvalue (`GameplayStatics.GetPlayerCharacter` 0))
  (bind _returnvalue_2 (`Actor.K2_GetActorLocation` _returnvalue))
  (bind (_outhit _returnvalue_3) (`KismetSystemLibrary.SphereTraceSingle` _returnvalue_2 (+ _returnvalue_2 (* (`Actor.GetActorForwardVector` _returnvalue) (`self.interaction range`))) 50.0 "TraceTypeQuery3" false (`|MakeArray` (`self.GetOwner`))))
  (if _returnvalue_3
    (bind (_bblockinghit _binitialoverlap _time _distance _location _impactpoint _normal _impactnormal _physmat _hitactor) (`GameplayStatics.BreakHitResult` _outhit))
    (if (!= _hitactor (`self.Look At actor`))
      (bind _output_get (set `self.Look At actor` _hitactor))
      (bind _message (message `/Game/Blueprint/Inventory/interactionInterface.lookAt` _output_get null))
      (`KismetSystemLibrary.PrintString` (`KismetTextLibrary.Conv_TextToString` _message)))
    (else
      (set `self.Look At actor` null))))

(fn `removeFromInventory`
  (params (Name :type Name) (Quantity :type Integer)))