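; BP_PuzzleMesh is a toggleable puzzle piece whose static mesh is shown or hidden according to its ActiveStatus.
; Switch flips the status unless the PuzzleManager is completed, then passes itself to the manager's Update.
; Affected flips the status without notifying the manager.
; The mesh visibility is applied in the construction script and refreshed every Tick.
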(event `self.ReceiveTick`
  (params (DeltaSeconds :type "Float (single-precision)"))
  (bind _staticmesh (`self.StaticMesh`))
  (if (`self.ActiveStatus`)
    (`SceneComponent.SetVisibility` _staticmesh true true)
    (else
      (`SceneComponent.SetVisibility` _staticmesh false true))))

(event `Switch`
  ;[1 1 1] Switch On/Off
  (if (not (`/Game/Blueprint/puzzle/BP_PuzzleManager.StatusCompleted` (`self.PuzzleManager`)))
    (set `self.ActiveStatus` (not (`self.ActiveStatus`)))
    (`/Game/Blueprint/puzzle/BP_PuzzleManager.Update` (`self.PuzzleManager`) self)))

(event `Affected`
  ;[1 1 1] Affected
  (set `self.ActiveStatus` (not (`self.ActiveStatus`))))

(fn `UserConstructionScript`
  (bind _staticmesh (`self.StaticMesh`))
  (if (`self.ActiveStatus`)
    (`SceneComponent.SetVisibility` _staticmesh true true)
    (else
      (`SceneComponent.SetVisibility` _staticmesh false true))))