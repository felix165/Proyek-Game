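; BP_puzOnHit is a puzzle Blueprint that tracks three stones through component hit events and prints a solved message.
; A shared hit handler sets the three destroyed flags in sequence, one per call, without checking which component was hit or destroying anything.
; The handler assigns itself to the stones' hit events from within its own body, with no initial binding in BeginPlay.
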(event `self.ReceiveBeginPlay`)

(event `OnComponentHit_Event_0`
  (params (HitComponent :type "PrimitiveComponent Object Reference") (OtherActor :type "Actor Object Reference") (OtherComp :type "PrimitiveComponent Object Reference") (NormalImpulse :type "Vector Structure") (Hit :type "HitResult Structure (by ref)"))
  (add `PrimitiveComponent.OnComponentHit` (`self.stone1`) (delegate `OnComponentHit_Event_0`))
  (if (`self.stone1_destroyed`)
    (add `PrimitiveComponent.OnComponentHit` (`self.stone2`) (delegate `OnComponentHit_Event_0`))
    (if (`self.stone2_destroyed`)
      (add `PrimitiveComponent.OnComponentHit` (`self.stone3`) (delegate `OnComponentHit_Event_0`))
      (if (not (`self.stone3_destroyed`))
        (set `self.stone3_destroyed` true)
        (if (and (`self.stone1_destroyed`) (`self.stone2_destroyed`) (`self.stone3_destroyed`)) :!label _label
          (`KismetSystemLibrary.PrintString` "puzzle solved")))
      (else
        (set `self.stone2_destroyed` true)
        (goto _label)))
    (else
      (set `self.stone1_destroyed` true)
      (goto _label))))

(fn `UserConstructionScript`)