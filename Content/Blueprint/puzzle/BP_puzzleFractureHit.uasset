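; Puzzle Blueprint that counts actor hits toward three destroyed flags, reporting "puzzle solved" once all are true.
; Each hit event sets the first unset flag in the Destroyed array, regardless of which actor was hit.
; The handler binds itself to OnActorHit on successive Puzzle actors as it runs, with no initial binding in these graphs.
; Progress and completion are only printed to screen.
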(event `OnActorHit_Event` :!signature `self.OnActorHit`
  (params (SelfActor :type "Actor Object Reference") (OtherActor :type "Actor Object Reference") (NormalImpulse :type "Vector Structure") (Hit :type "HitResult Structure (by ref)"))
  (bind _puzzle (`self.puzzle`))
  (bind _destroyed (`self.destroyed`))
  (bind _output (`|GetArrayItem` _destroyed 2))
  (bind _output_2 (`|GetArrayItem` _destroyed))
  (bind _output_3 (`|GetArrayItem` _destroyed 1))
  (bind _returnvalue (and _output_2 _output_3 _output))
  (add `self.OnActorHit` (`|GetArrayItem` _puzzle) (delegate `OnActorHit_Event`))
  (if _output_2
    (add `self.OnActorHit` (`|GetArrayItem` _puzzle 1) (delegate `OnActorHit_Event`))
    (if _output_3
      (add `self.OnActorHit` (`|GetArrayItem` _puzzle 2) (delegate `OnActorHit_Event`))
      (if (not _output)
        (`KismetArrayLibrary.Array_Set` _destroyed 2 true)
        (`KismetSystemLibrary.PrintString` (`KismetStringLibrary.Conv_BoolToString` _returnvalue) :!label _label)
        (if _returnvalue
          (`KismetSystemLibrary.PrintString` "puzzle solved")))
      (else
        (`KismetArrayLibrary.Array_Set` _destroyed 1 true)
        (goto _label)))
    (else
      (`KismetArrayLibrary.Array_Set` _destroyed 0 true)
      (goto _label))))

(fn `UserConstructionScript`)