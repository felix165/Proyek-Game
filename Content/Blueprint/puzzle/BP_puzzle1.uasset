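; Puzzle actor in which the player removes three stones by stepping into each stone's box, in any order.
; Tick polls the three boxes in an if/else chain for overlap with the player character, destroying the matching stone component once and setting its flag.
; After each removal it checks all three flags and, when all are set, only prints a "puzzle solved" message.
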(event `self.ReceiveBeginPlay`)

(event `self.ReceiveTick`
  (params (DeltaSeconds :type "Float (single-precision)"))
  (if (`PrimitiveComponent.IsOverlappingActor` (`self.box_stone1`) (`GameplayStatics.GetPlayerCharacter` 0))
    (if (not (`self.stone1_destroyed`))
      (set `self.stone1_destroyed` true)
      (`ActorComponent.K2_DestroyComponent` (`self.stone1`))
      (if (and (`self.stone1_destroyed`) (`self.stone2_destroyed`) (`self.stone3_destroyed`)) :!label _label
        (`KismetSystemLibrary.PrintString` "puzzle solved")))
    (elif (`PrimitiveComponent.IsOverlappingActor` (`self.box_stone2`) (`GameplayStatics.GetPlayerCharacter` 0))
      (if (not (`self.stone2_destroyed`))
        (set `self.stone2_destroyed` true)
        (`ActorComponent.K2_DestroyComponent` (`self.stone2`))
        (goto _label))
      (elif (`self.stone3_destroyed`)
        _
        (elif (`PrimitiveComponent.IsOverlappingActor` (`self.box_stone3`) (`GameplayStatics.GetPlayerCharacter` 0))
          (set `self.stone3_destroyed` true)
          (`ActorComponent.K2_DestroyComponent` (`self.stone3`))
          (goto _label))))))

(fn `UserConstructionScript`)