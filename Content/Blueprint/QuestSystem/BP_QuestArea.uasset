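; BP_QuestArea is a quest objective actor that checks each tick, until completed, whether its objective is met.
; QuestUpdate switches on QuestType: counting invalid references in EnemiesToDefeat, testing player distance to the actor, or reading BP_VeteranHunter's dialog progress.
; Completion sets Completed and clears NeedToNav; location and dialog quests also deactivate the particle system, which starts off, and dialog quests disable the hunter's interaction.
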(event `self.ReceiveBeginPlay`
  (`ActorComponent.Deactivate` (`self.ParticleSystem`)))

(event `self.ReceiveActorBeginOverlap`
  (params (OtherActor :type "Actor Object Reference")))

(event `self.ReceiveTick`
  (params (DeltaSeconds :type "Float (single-precision)"))
  (`self.QuestUpdate`))

(fn `QuestUpdate`
  (if (not (`self.Completed`))
    (switch `/Game/Blueprint/Information/Enum_QuestType` (`self.QuestType`)
      (:`NewEnumerator0`
        ;[1 1 1] Defeat Enemy Counter
        (set `self.Enemies_Counter` 0)
        (for _array_element (`self.EnemiesToDefeat`)
          (bind _asbp_enemies_base (cast `/Game/Blueprint/Characters/Character/Enemy/BP_EnemiesBase` _array_element))
          (`/Engine/EditorBlueprintResources/StandardMacros.IsValid` _asbp_enemies_base
            (:`Is Not Valid`
              (bind _result (`/Engine/EditorBlueprintResources/StandardMacros.IncrementInt` (`self.Enemies_Counter`))
                (:`  `
                  (if (== _result (`KismetArrayLibrary.Array_Length` (`self.EnemiesToDefeat`)))
                    (set `self.Completed` true)
                    (set `self.NeedToNav?` false))))))))
      (:`NewEnumerator1`
        ;[1 1 1] Go To Specific Location
        (if (< (`self.GetDistanceTo` (`GameplayStatics.GetPlayerCharacter` 0) self) 400.0)
          (set `self.Completed` true)
          (`ActorComponent.Deactivate` (`self.ParticleSystem`))
          (set `self.NeedToNav?` false)))
      (:`NewEnumerator2`
        (bind _returnvalue (`GameplayStatics.GetActorOfClass` "/Game/Blueprint/Characters/Character/Bystander/Veteran_Hunter/BP_VeteranHunter.BP_VeteranHunter_C"))
        (if (>= (`/Game/Blueprint/Characters/Character/Bystander/Veteran_Hunter/BP_VeteranHunter.CurrentDialog` _returnvalue) (`/Game/Blueprint/Characters/Character/Bystander/Veteran_Hunter/BP_VeteranHunter.Finish` _returnvalue))
          (set `self.Completed` true)
          (`ActorComponent.Deactivate` (`self.ParticleSystem`))
          (set `self.NeedToNav?` false)
          (set `/Game/Blueprint/Characters/Character/Bystander/Veteran_Hunter/BP_VeteranHunter.canInteract` false _returnvalue))))))

(fn `UserConstructionScript`)