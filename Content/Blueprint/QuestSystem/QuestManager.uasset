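; Quest manager that runs the main quest line as a linear sequence from the Quests array.
; On BeginPlay it clears every quest's NeedToNav flag, then activates the first quest.
; Tick polls the current quest's Completed flag and advances the index to activate the next one.
; Activation sets NeedToNav and, for Go to Location quests only, turns on the quest's particle system; other types have no extra logic.
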(event `self.ReceiveBeginPlay`
  (`|ExecutionSequence`
    (:`then_0`
      (for _array_element (`self.Quests`)
        (set `/Game/AdvWorldInteraction/Blueprints/Areas/BP_NavPoint.NeedToNav?` false _array_element)))
    (:`then_1`
      (bind _output_get (set `self.CurrentQuests` 0))
      (`self.Activate Quests` _output_get))))

(event `self.ReceiveTick`
  (params (DeltaSeconds :type "Float (single-precision)"))
  (`self.Update Main Quest`))

(fn `Activate Quests`
  (params (`Current Quest` :type Integer))
  (bind _output (`|GetArrayItem` (`self.Quests`) `Current Quest`))
  (`/Engine/EditorBlueprintResources/StandardMacros.IsValid` _output
    (:`Is Valid`
      (switch `/Game/Blueprint/Information/Enum_QuestType` (`/Game/Blueprint/QuestSystem/BP_QuestArea.QuestType` _output)
        (:`NewEnumerator0`
          _)
        (:`NewEnumerator1`
          (`ActorComponent.Activate` (`/Game/Blueprint/QuestSystem/BP_QuestArea.ParticleSystem` _output) true))
        (:`NewEnumerator2`
          _))
      (set `/Game/AdvWorldInteraction/Blueprints/Areas/BP_NavPoint.NeedToNav?` true _output))))

(fn `Update Main Quest`
  (bind _output (`|GetArrayItem` (`self.Quests`) (`self.CurrentQuests`)))
  (`/Engine/EditorBlueprintResources/StandardMacros.IsValid` _output
    (:`Is Valid`
      (if (`/Game/Blueprint/QuestSystem/BP_QuestArea.Completed` _output)
        (bind _result (`/Engine/EditorBlueprintResources/StandardMacros.IncrementInt` (`self.CurrentQuests`))
          (:`  `
            (`self.Activate Quests` _result)))))))

(fn `UserConstructionScript`)