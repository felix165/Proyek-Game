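; BP_stone1 is a lights-out style puzzle of three glowing stones, solved when all three are lit.
; Player character overlap or the shot event checks which Puzzle1 box the player overlaps, toggling Lighted flags and purple/marble materials on Stone's slots.
; The middle entry toggles all three with delays between them, and the last toggles itself and the middle, then both print solved status.
; The first only flips its flag; its material and neighbor logic is disconnected.
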(event `self.ReceiveActorBeginOverlap`
  (params (OtherActor :type "Actor Object Reference"))
  (bind _returnvalue (`GameplayStatics.GetPlayerCharacter` 0))
  (bind _stone (`self.stone`))
  (bind _lighted (`self.lighted`))
  (bind _lighted_2 (`self.lighted`))
  (bind _lighted_3 (`self.lighted`))
  (bind _lighted_4 (`self.lighted`))
  (bind _puzzle1 (`self.puzzle1`))
  (bind _stone_2 (`self.stone`))
  (bind _lighted_5 (`self.lighted`))
  (cast `/Game/ThirdPerson/Blueprints/BP_ThirdPersonCharacter` OtherActor)
  (`|ExecutionSequence` :!label _label
    (:`then_0`
      (if (`PrimitiveComponent.IsOverlappingActor` (`/Game/Blueprint/Assets/puzzle/BP_stone1.Box` (`|GetArrayItem` _puzzle1)) _returnvalue)
        (if (`|GetArrayItem` _lighted)
          (`KismetArrayLibrary.Array_Set` _lighted)
          (else
            (`KismetArrayLibrary.Array_Set` _lighted 0 true)))))
    (:`then_1`
      (if (`PrimitiveComponent.IsOverlappingActor` (`/Game/Blueprint/Assets/puzzle/BP_stone1.Box` (`|GetArrayItem` _puzzle1 1)) _returnvalue)
        (if (`|GetArrayItem` _lighted_2 1)
          (`KismetArrayLibrary.Array_Set` _lighted_2 1)
          (`PrimitiveComponent.SetMaterial` _stone 1 "/Game/Blueprint/Assets/puzzle/stone_asset/stylized-glowing-rock/textures/stone_glow_marble.stone_glow_marble")
          (`KismetSystemLibrary.Delay` 2.0)
          (else
            (`KismetArrayLibrary.Array_Set` _lighted_2 1 true)
            (`PrimitiveComponent.SetMaterial` _stone 1 "/Game/Blueprint/Assets/puzzle/stone_asset/stylized-glowing-rock/textures/stone_glow_purple.stone_glow_purple")
            (`KismetSystemLibrary.Delay` 2.0)))
        (if (`|GetArrayItem` _lighted_2)
          (`KismetArrayLibrary.Array_Set` _lighted_2)
          (`PrimitiveComponent.SetMaterial` _stone 0 "/Game/Blueprint/Assets/puzzle/stone_asset/stylized-glowing-rock/textures/stone_glow_marble.stone_glow_marble")
          (`KismetSystemLibrary.Delay` 1.0)
          (else
            (`KismetArrayLibrary.Array_Set` _lighted_2 0 true)
            (`PrimitiveComponent.SetMaterial` _stone 0 "/Game/Blueprint/Assets/puzzle/stone_asset/stylized-glowing-rock/textures/stone_glow_purple.stone_glow_purple")
            (`KismetSystemLibrary.Delay` 1.0)))
        (if (`|GetArrayItem` _lighted_2 2)
          (`KismetArrayLibrary.Array_Set` _lighted_2 2)
          (`PrimitiveComponent.SetMaterial` _stone 2 "/Game/Blueprint/Assets/puzzle/stone_asset/stylized-glowing-rock/textures/stone_glow_marble.stone_glow_marble")
          (else
            (`KismetArrayLibrary.Array_Set` _lighted_2 2 true)
            (`PrimitiveComponent.SetMaterial` _stone 2 "/Game/Blueprint/Assets/puzzle/stone_asset/stylized-glowing-rock/textures/stone_glow_purple.stone_glow_purple")))
        (if (and (`|GetArrayItem` _lighted_5) (`|GetArrayItem` _lighted_5 1) (`|GetArrayItem` _lighted_5 2)) :!label _label_2
          (`KismetSystemLibrary.PrintString` "puzzle solved")
          (else
            (`KismetSystemLibrary.PrintString` "puzzle not solved")))))
    (:`then_2`
      (if (`PrimitiveComponent.IsOverlappingActor` (`/Game/Blueprint/Assets/puzzle/BP_stone1.Box` (`|GetArrayItem` _puzzle1 2)) _returnvalue)
        (if (`|GetArrayItem` _lighted_3 2)
          (`KismetArrayLibrary.Array_Set` _lighted_3 2)
          (`PrimitiveComponent.SetMaterial` _stone_2 2 "/Game/Blueprint/Assets/puzzle/stone_asset/stylized-glowing-rock/textures/stone_glow_marble.stone_glow_marble")
          (else
            (`KismetArrayLibrary.Array_Set` _lighted_3 2 true)
            (`PrimitiveComponent.SetMaterial` _stone_2 2 "/Game/Blueprint/Assets/puzzle/stone_asset/stylized-glowing-rock/textures/stone_glow_purple.stone_glow_purple")))
        (if (`|GetArrayItem` _lighted_4 1)
          (`KismetArrayLibrary.Array_Set` _lighted_4 1)
          (`PrimitiveComponent.SetMaterial` _stone_2 1 "/Game/Blueprint/Assets/puzzle/stone_asset/stylized-glowing-rock/textures/stone_glow_marble.stone_glow_marble")
          (goto _label_2)
          (else
            (`KismetArrayLibrary.Array_Set` _lighted_4 1 true)
            (`PrimitiveComponent.SetMaterial` _stone_2 1 "/Game/Blueprint/Assets/puzzle/stone_asset/stylized-glowing-rock/textures/stone_glow_purple.stone_glow_purple")
            (goto _label_2)))))))

(event `shot`
  (goto _label))

(fn `UserConstructionScript`)