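; BP_puzzleFracture tracks a three-piece puzzle that is solved once the player has touched every piece, in any order.
; Each Tick it checks player 0's character against the Box of the three Puzzle entries in an if-else chain.
; A first overlap sets that piece's Destroyed flag, then prints whether all three are set and "puzzle solved" when they are.
; Only flags and debug prints change here, with no fracture logic.
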(event `self.ReceiveTick`
  (params (DeltaSeconds :type "Float (single-precision)"))
  (bind _returnvalue (`GameplayStatics.GetPlayerCharacter` 0))
  (bind _puzzle (`self.puzzle`))
  (bind _destroyed (`self.destroyed`))
  (bind _output (`|GetArrayItem` _destroyed 2))
  (bind _output_2 (`|GetArrayItem` _destroyed))
  (bind _output_3 (`|GetArrayItem` _destroyed 1))
  (bind _returnvalue_2 (and _output_2 _output_3 _output))
  (if (`PrimitiveComponent.IsOverlappingActor` (`/Game/Blueprint/Assets/puzzle/BP_puzzleFracture.Box` (`|GetArrayItem` _puzzle)) _returnvalue)
    (if (not _output_2)
      (`KismetArrayLibrary.Array_Set` _destroyed 0 true)
      (`KismetSystemLibrary.PrintString` (`KismetStringLibrary.Conv_BoolToString` _returnvalue_2) :!label _label)
      (if _returnvalue_2
        (`KismetSystemLibrary.PrintString` "puzzle solved")))
    (elif (`PrimitiveComponent.IsOverlappingActor` (`/Game/Blueprint/Assets/puzzle/BP_puzzleFracture.Box` (`|GetArrayItem` _puzzle 1)) _returnvalue)
      (if (not _output_3)
        (`KismetArrayLibrary.Array_Set` _destroyed 1 true)
        (goto _label))
      (elif (`PrimitiveComponent.IsOverlappingActor` (`/Game/Blueprint/Assets/puzzle/BP_puzzleFracture.Box` (`|GetArrayItem` _puzzle 2)) _returnvalue)
        (if (not _output)
          (`KismetArrayLibrary.Array_Set` _destroyed 2 true)
          (goto _label))))))

(fn `UserConstructionScript`)