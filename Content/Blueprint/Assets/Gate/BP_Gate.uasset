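; BP_Gate is a gate actor that slides its Gate component along one axis when key 3 is pressed.
; A Selection value picks the direction: Atas Bawah (up/down) drives Z through Timeline_gate, and Kanan Kiri (right/left) drives X through Timeline_0.
; Each timeline's GateTrack, scaled by HeightSpeed, sets the relative location.
; Timelines only play forward, with no closing logic.
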(event `Key|Three`
  (params (Key :type "Key Structure"))
  (:`Pressed`
    (switch `/Game/Blueprint/Assets/Gate/gateDirection` (`self.Selection`)
      (:`NewEnumerator0`
        (bind (_direction _gate_track) (`Timeline|Timeline_gate`)
          (:`Update`
            (`SceneComponent.K2_SetRelativeLocation` (`self.gate`) (`KismetMathLibrary.MakeVector` 0.0 0.0 (* _gate_track (`self.height & speed`))) false false))))
      (:`NewEnumerator1`
        (bind (_direction_2 _gate_track_2) (`Timeline|Timeline_0`)
          (:`Update`
            (`SceneComponent.K2_SetRelativeLocation` (`self.gate`) (`KismetMathLibrary.MakeVector` (* _gate_track_2 (`self.height & speed`))) false false)))))))

(fn `UserConstructionScript`)