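; BP_puzzle2 is an unfinished Blueprint for what appears to be a light-up stone puzzle with two box stones.
; Each Tick it checks whether the player character overlaps BoxStone1, but nothing follows from the result.
; Disconnected loops over the light-up flags and stone materials are left in the graph and never run.
; The construction script is empty.
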(event `self.ReceiveTick`
  (params (DeltaSeconds :type "Float (single-precision)"))
  (if (`PrimitiveComponent.IsOverlappingActor` (`self.box_stone1`) (`GameplayStatics.GetPlayerCharacter` 0))
    _))

(fn `UserConstructionScript`)