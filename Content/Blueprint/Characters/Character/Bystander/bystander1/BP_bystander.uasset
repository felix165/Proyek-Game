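; Bystander character that moves by AI toward placed location markers, then changes its look and removes itself from the level.
; BeginPlay caches three locations and chains AIMoveTo calls on their immediate exec pins, so all three requests fire back-to-back without waiting for arrival.
; Success of the last move swaps the mesh materials, waits briefly and destroys the actor.
; The Tick distance check does nothing, and random-point selection is not called here.
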(event `self.ReceiveTick`
  (params (DeltaSeconds :type "Float (single-precision)"))
  (if (< (`KismetMathLibrary.Vector_Distance` (`SceneComponent.K2_GetComponentLocation` (`self.CapsuleComponent`)) (`self.curr target`)) 1.0)
    _))

(event `self.ReceiveBeginPlay`
  (bind _mesh (`self.Mesh`))
  (bind _output_get (set `self.patrol` (`|MakeArray` (`SceneComponent.K2_GetComponentLocation` (`self.loc1`)) (`SceneComponent.K2_GetComponentLocation` (`self.loc2`)) (`SceneComponent.K2_GetComponentLocation` (`self.loc3`)))))
  (`|AIMoveTo` self (`|GetArrayItem` _output_get) null
    (:`then`
      (`|AIMoveTo` self (`|GetArrayItem` _output_get 1) null
        (:`then`
          (`|AIMoveTo` self (`|GetArrayItem` _output_get 2) null
            (:`OnSuccess`
              (`PrimitiveComponent.SetMaterial` _mesh 0 "/Game/Blueprint/Characters/Character/Bystander/bystander1/Ch35_body_Inst.Ch35_body_Inst")
              (`PrimitiveComponent.SetMaterial` _mesh 1 "/Game/Blueprint/Characters/Character/Bystander/bystander1/Ch35_body_Inst.Ch35_body_Inst")
              (`PrimitiveComponent.SetMaterial` _mesh 2 "/Game/Blueprint/Characters/Character/Bystander/bystander1/Ch35_body_Inst.Ch35_body_Inst")
              (`KismetSystemLibrary.Delay` 5.0)
              (`self.K2_DestroyActor`))))))))

(fn `get loc`
  (set `self.cur patrol loc` (`KismetMathLibrary.RandomInteger` (`KismetArrayLibrary.Array_Length` (`self.patrol`)))))

(fn `UserConstructionScript`)