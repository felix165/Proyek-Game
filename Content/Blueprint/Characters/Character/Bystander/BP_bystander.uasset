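; BP_bystander is a bystander character that wanders between three patrol points.
; BeginPlay caches the world locations of its three location components into a patrol array.
; Tick plays the Walk timeline, whose updates issue AI move requests to a point a tenth of the way toward the current patrol point.
; When the timeline finishes, a short delay precedes a random pick of the next point.
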(event `self.ReceiveTick`
  (params (DeltaSeconds :type "Float (single-precision)"))
  (`Timeline|walk`
    (:`Update`
      (`|AIMoveTo` null (`KismetMathLibrary.VLerp` (`self.K2_GetActorLocation`) (`|GetArrayItem` (`self.patrol`) (`self.cur patrol loc`)) 0.1) null))
    (:`Finished`
      (`KismetSystemLibrary.Delay` 0.5)
      (`self.get loc`))))

(event `self.ReceiveBeginPlay`
  (set `self.patrol` (`|MakeArray` (`SceneComponent.K2_GetComponentLocation` (`self.loc1`)) (`SceneComponent.K2_GetComponentLocation` (`self.loc2`)) (`SceneComponent.K2_GetComponentLocation` (`self.loc3`)))))

(fn `get loc`
  (set `self.cur patrol loc` (`KismetMathLibrary.RandomInteger` (`KismetArrayLibrary.Array_Length` (`self.patrol`)))))

(fn `UserConstructionScript`)