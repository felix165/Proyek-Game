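; BP_VeteranHunter is a bystander NPC that the player can interact with to start a dialog.
; On BeginPlay it finds and stores a reference to the level's QuestManager, which this graph does not otherwise use.
; Interact checks CanInteract, sets an IsDialog flag to block re-entry, then deactivates the Twinblast player's character movement and shows the mouse cursor.
; The graph contains no logic to display dialog content or end the dialog.
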(event EventBeginPlay
  (bind _returnvalue (Actor|GetActorOfClass "/Game/Blueprint/QuestSystem/QuestManager.QuestManager_C"))
  (Variables|Default|SetQManager _returnvalue))

(event Collision|EventActorBeginOverlap
  (params (OtherActor :type Actor%20Object%20Reference)))

(event EventTick
  (params (DeltaSeconds :type Float%20%28single-precision%29)))

(event EventInteract
  (if (Variables|Default|GetcanInteract)
    (if (not (Variables|Default|GetisDialog))
      (bind _output_get (Variables|Default|SetisDialog true))
      (if _output_get
        (bind _astwinblast_player_character (Utilities|Casting|CastToTwinblastPlayerCharacter (Game|GetPlayerCharacter 0)))
        (Components|Activation|Deactivate (Variables|/Script/Engine.Character|GetCharacterMovement _astwinblast_player_character))
        (Variables|/Script/Engine.PlayerController|SetbShowMouseCursor (Game|GetPlayerController 0) true)))))

(fn ConstructionScript)