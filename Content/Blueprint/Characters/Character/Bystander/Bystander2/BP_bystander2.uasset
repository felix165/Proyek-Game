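; Bystander character Blueprint that sends itself toward patrol points when play begins, with no looping.
; BeginPlay stores the world locations of Loc1, Loc2 and Loc3 in a Patrol array, then issues an AI MoveTo for each in order.
; The moves chain from the immediate Then output rather than On Success, so they do not wait for arrival.
; Tick, overlap and construction logic are empty.
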(event `self.ReceiveBeginPlay`
  (bind _output_get (set `self.patrol` (`|MakeArray` (`SceneComponent.K2_GetComponentLocation` (`self.loc1`)) (`SceneComponent.K2_GetComponentLocation` (`self.loc2`)) (`SceneComponent.K2_GetComponentLocation` (`self.loc3`)))))
  (`|AIMoveTo` self (`|GetArrayItem` _output_get) null
    (:`then`
      (`|AIMoveTo` self (`|GetArrayItem` _output_get 1) null
        (:`then`
          (`|AIMoveTo` self (`|GetArrayItem` _output_get 2) null))))))

(fn `UserConstructionScript`)