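; BP_Status1 is a character status Blueprint that creates a set of ability actors when flagged as a player.
; On BeginPlay, if IsPlayer is true, it spawns BasicAttack, Recovery, PowerUp and Balistic actors at its own transform.
; Each spawned actor is stored in a matching variable, and the Blueprint has no other active logic.
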(event `self.ReceiveBeginPlay`
  (bind _returnvalue (`self.GetTransform` self))
  (if (`self.isPlayer`)
    (bind _returnvalue_2 (`|SpawnActorFromClass` "/Game/Blueprint/Characters/Character/Skill/BP_BasicAttack.BP_BasicAttack_C" _returnvalue "Undefined" "OverrideRootScale" null null))
    (set `self.BasicAttack` _returnvalue_2)
    (bind _returnvalue_3 (`|SpawnActorFromClass` "/Game/Blueprint/Characters/Character/Skill/BP_Recovery.BP_Recovery_C" _returnvalue "Undefined" "OverrideRootScale" null null))
    (set `self.Recovery` _returnvalue_3)
    (bind _returnvalue_4 (`|SpawnActorFromClass` "/Game/Blueprint/Characters/Character/Skill/BP_PowerUp.BP_PowerUp_C" _returnvalue "Undefined" "OverrideRootScale" null null))
    (set `self.PowerUp` _returnvalue_4)
    (bind _returnvalue_5 (`|SpawnActorFromClass` "/Game/Blueprint/Characters/Character/Skill/BP_Balistic.BP_Balistic_C" _returnvalue "Undefined" "OverrideRootScale" null null))
    (set `self.Balistic` _returnvalue_5)))

(fn `UserConstructionScript`)