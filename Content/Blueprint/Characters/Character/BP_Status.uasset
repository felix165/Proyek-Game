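; BP_Status is an actor that holds a character's stats and skills and handles level-ups for the player.
; InitializeSkill spawns five skill actors (BasicAttack, Recovery, PowerUp, Blastic, FatalShot) and stores references to them.
; Stat events raise Health, Energy, Defense, Attack or Evasion, with Health and Energy also boosting regeneration and refilling.
; Skill events forward LevelUp to their actors, as does Attack for BasicAttack; every upgrade requires IsPlayer.
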(event `self.ReceiveBeginPlay`)

(event `InitializeSkill`
  (bind _returnvalue (`self.GetTransform` self))
  (if (`self.isPlayer`)
    (bind _returnvalue_2 (`|SpawnActorFromClass` "/Game/Blueprint/Characters/Character/Skill/BP_BasicAttack.BP_BasicAttack_C" _returnvalue "Undefined" "OverrideRootScale" null null))
    (set `self.BasicAttack` _returnvalue_2)
    (bind _returnvalue_3 (`|SpawnActorFromClass` "/Game/Blueprint/Characters/Character/Skill/BP_Recovery.BP_Recovery_C" _returnvalue "Undefined" "OverrideRootScale" null null))
    (set `self.Recovery` _returnvalue_3)
    (bind _returnvalue_4 (`|SpawnActorFromClass` "/Game/Blueprint/Characters/Character/Skill/BP_PowerUp.BP_PowerUp_C" _returnvalue "Undefined" "OverrideRootScale" null null))
    (set `self.PowerUp` _returnvalue_4)
    (bind _returnvalue_5 (`|SpawnActorFromClass` "/Game/Blueprint/Characters/Character/Skill/BP_Blastic.BP_Blastic_C" _returnvalue "Undefined" "OverrideRootScale" null null))
    (set `self.Blastic` _returnvalue_5)
    (bind _returnvalue_6 (`|SpawnActorFromClass` "/Game/Blueprint/Characters/Character/Skill/BP_FatalShot.BP_FatalShot_C" _returnvalue "Undefined" "OverrideRootScale" null null))
    (set `self.FatalShot` _returnvalue_6)))

(event `LevelUpHealth`
  (if (`self.isPlayer`)
    (`/Engine/EditorBlueprintResources/StandardMacros.IncrementFloat` (`self.HealthLevel`)
      (:`  `
        (bind _output_get (set `self.MaxHealth` (+ (`self.HealthUpBase`) (`self.MaxHealth`))))
        (set `self.HealthRegenPerSec` (+ (`self.HealthRegenPerSec`) 5.0))
        (set `self.Health` _output_get)))))

(event `LevelUpEnergy`
  (if (`self.isPlayer`)
    (`/Engine/EditorBlueprintResources/StandardMacros.IncrementFloat` (`self.EnergyLevel`)
      (:`  `
        (bind _output_get (set `self.MaxEnergy` (+ (`self.EnergyUpBase`) (`self.MaxEnergy`))))
        (set `self.EnergyRegenPerSec` (+ (`self.EnergyRegenPerSec`) 4.0))
        (set `self.Energy` _output_get)))))

(event `LevelUpDefense`
  (if (`self.isPlayer`)
    (`/Engine/EditorBlueprintResources/StandardMacros.IncrementFloat` (`self.DefenseLevel`)
      (:`  `
        (set `self.Defense` (+ (`self.DefenseUpBase`) (`self.Defense`)))))))

(event `LevelUpAttack`
  (if (`self.isPlayer`)
    (`/Game/Blueprint/Characters/Character/Skill/BP_BasicAttack.LevelUp` (`self.BasicAttack`))
    (set `self.Attack` (+ (`self.AttackUpBase`) (`self.Attack`)))))

(event `LevelUpEvasion`
  (if (`self.isPlayer`)
    (`/Engine/EditorBlueprintResources/StandardMacros.IncrementFloat` (`self.EvasionLevel`)
      (:`  `
        (set `self.EvasionRate` (+ (`self.EvasionUpBase`) (`self.EvasionRate`)))))))

(event `LevelUpFatalShot`
  (if (`self.isPlayer`)
    (`/Game/Blueprint/Characters/Character/Skill/BP_FatalShot.LevelUp` (`self.FatalShot`))))

(event `LevelUpPowerUp`
  (if (`self.isPlayer`)
    (`/Game/Blueprint/Characters/Character/Skill/BP_PowerUp.LevelUp` (`self.PowerUp`))))

(event `LevelUpBlastic`
  (if (`self.isPlayer`)
    (`/Game/Blueprint/Characters/Character/Skill/BP_Blastic.LevelUp` (`self.Blastic`))))

(event `LevelUpRecovery`
  (if (`self.isPlayer`)
    (`/Game/Blueprint/Characters/Character/Skill/BP_Recovery.LevelUp` (`self.Recovery`))))

(fn `UserConstructionScript`)