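; Base enemy Blueprint that gives enemies combat stats and two-way damage with the Twinblast player character.
; On BeginPlay it spawns a BP_Status actor to hold health, energy, attack and defense.
; Tick writes IsDead to the AI blackboard and raises attack once health drops to a threshold.
; HitEnemy subtracts damage minus defense from health, unclamped, while HitPlayer applies the attack stat as damage to the player.
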(event Custom|HitEnemy
  (params (PlayerDamage :type Float%20%28double-precision%29))
  (CallFunction|HItEnemyCalculation PlayerDamage))

(event EventBeginPlay
  (bind _returnvalue (Game|SpawnActorfromClass "/Game/Blueprint/Characters/Character/BP_Status.BP_Status_C" (Transformation|GetActorTransform) "Undefined" 0 0))
  (bind _output_get (Variables|Default|SetStatuss _returnvalue))
  (Utilities|FlowControl|Sequence
    (:then_0
      (bind _output_get_2 (Variables|/Game/Blueprint/Characters/Character/BP_Status.BP_Status_C|SetMaxHealth _output_get 3e+02))
      (Variables|/Game/Blueprint/Characters/Character/BP_Status.BP_Status_C|SetHealth _output_get _output_get_2))
    (:then_1
      (bind _output_get_3 (Variables|/Game/Blueprint/Characters/Character/BP_Status.BP_Status_C|SetMaxEnergy _output_get 0.0))
      (Variables|/Game/Blueprint/Characters/Character/BP_Status.BP_Status_C|SetEnergy _output_get _output_get_3)
      (Variables|/Game/Blueprint/Characters/Character/BP_Status.BP_Status_C|SetEnergyRegenPerSec _output_get _output_get_3))
    (:then_2
      (Variables|/Game/Blueprint/Characters/Character/BP_Status.BP_Status_C|SetAttack _output_get 1e+02))
    (:then_3
      (Variables|/Game/Blueprint/Characters/Character/BP_Status.BP_Status_C|SetDefense _output_get 1e+01))))

(event Collision|EventActorBeginOverlap
  (params (OtherActor :type Actor%20Object%20Reference)))

(event EventTick
  (params (DeltaSeconds :type Float%20%28single-precision%29))
  (bind _statuss (Variables|Default|GetStatuss))
  (AI|Components|Blackboard|SetValueasBool (AI|GetBlackboard 0) (Utilities|Name|MakeLiteralName "IsDead") (== (Math|Float|Max(Float) (Variables|/Game/Blueprint/Characters/Character/BP_Status.BP_Status_C|GetHealth (Variables|Default|GetStatuss)) 0.0) 0.0))
  (if (<= (Variables|/Game/Blueprint/Characters/Character/BP_Status.BP_Status_C|GetHealth _statuss) 2.5e+02)
    (Variables|/Game/Blueprint/Characters/Character/BP_Status.BP_Status_C|SetAttack _statuss 2e+02)))

(fn ConstructionScript)

(fn HitPlayer
  (params (Object :type Actor%20Object%20Reference))
  (bind _astwinblast_player_character (Utilities|Casting|CastToTwinblastPlayerCharacter Object))
  (Game|Damage|ApplyDamage _astwinblast_player_character (Variables|/Game/Blueprint/Characters/Character/BP_Status.BP_Status_C|GetAttack (Variables|Default|GetStatuss)) 0 0))

(fn HItEnemyCalculation
  (params (A :type Float%20%28double-precision%29))
  (bind _statuss (Variables|Default|GetStatuss))
  (Variables|/Game/Blueprint/Characters/Character/BP_Status.BP_Status_C|SetHealth _statuss (- (Variables|/Game/Blueprint/Characters/Character/BP_Status.BP_Status_C|GetHealth _statuss) (- A (Variables|/Game/Blueprint/Characters/Character/BP_Status.BP_Status_C|GetDefense _statuss)))))