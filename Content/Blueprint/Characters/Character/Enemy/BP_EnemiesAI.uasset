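; AI controller for enemy pawns that runs the BT_Enemies behavior tree and caches the controlled BP_Enemies pawn.
; AI perception writes whether BP_ThirdPersonCharacter is sensed to the CanSeePlayer blackboard key as a bool.
; Tick measures the distance from the pawn to the TargetLocation key, prints it, and writes it as a float under the same CanSeePlayer key name.
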(event `self.ReceiveBeginPlay`
  (`self.RunBehaviorTree` "/Game/Blueprint/Characters/Character/Enemy/BT_Enemies.BT_Enemies")
  (bind _asbp_enemies (cast `/Game/Blueprint/Characters/Character/Enemy/BP_Enemies` (`self.K2_GetPawn`)))
  (set `self.MyPawn` _asbp_enemies))

(event `self.AIPerception.OnTargetPerceptionUpdated`
  (params (Actor :type "Actor Object Reference") (Stimulus :type "AIStimulus Structure"))
  (cast `/Game/ThirdPerson/Blueprints/BP_ThirdPersonCharacter` Actor)
  (`BlackboardComponent.SetValueAsBool` (`AIBlueprintHelperLibrary.GetBlackboard` null) "CanSeePlayer" (`.bSuccessfullySensed` (break `AIStimulus` Stimulus))))

(event `self.ReceiveTick`
  (params (DeltaSeconds :type "Float (single-precision)"))
  (bind _returnvalue (`KismetMathLibrary.Vector_Distance` (`BlackboardComponent.GetValueAsVector` (`AIBlueprintHelperLibrary.GetBlackboard` null) "TargetLocation") (`self.K2_GetActorLocation` (`self.MyPawn`))))
  (`BlackboardComponent.SetValueAsFloat` (`AIBlueprintHelperLibrary.GetBlackboard` null) "CanSeePlayer" _returnvalue)
  (`KismetSystemLibrary.PrintString` (`KismetStringLibrary.Conv_DoubleToString` _returnvalue)))

(fn `UserConstructionScript`)