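; BP_Skeleton4 is a skeleton enemy character that sets its own health, defense and attack at BeginPlay.
; Melee attacks play a montage with delayed sound, while the sword collider's overlap calls HitPlayer.
; Incoming hits run damage calculation and count toward a third-hit stun, gated by TriggerStun, that briefly disables movement with Niagara feedback.
; Death clears TriggerStun, disables collision, plays montage, sounds and particles, then destroys the actor.
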(event `self.ReceiveBeginPlay`
  (bind _statuss (`self.Statuss`))
  (`parent.ReceiveBeginPlay`)
  (`|ExecutionSequence`
    (:`then_0`
      (bind _output_get (set `/Game/Blueprint/Characters/Character/BP_Status.MaxHealth` 500.0 _statuss))
      (set `/Game/Blueprint/Characters/Character/BP_Status.Health` _output_get _statuss))
    (:`then_1`
      (set `/Game/Blueprint/Characters/Character/BP_Status.Defense` 20.0 _statuss))
    (:`then_2`
      (set `/Game/Blueprint/Characters/Character/BP_Status.Attack` 175.0 _statuss))))

(event `self.ReceiveTick`
  (params (DeltaSeconds :type "Float (single-precision)"))
  (`parent.ReceiveTick` DeltaSeconds))

(event `/Game/Blueprint/Characters/Character/Enemy/CombatInterface.MeleeAttack`
  (`|PlayMontage` (`self.Mesh`) "/Game/CityofBrass_Enemies/Meshes/Enemy/Corpse/animation/SkeletonAttack4.SkeletonAttack4"
    (:`then`
      (`KismetSystemLibrary.Delay` 0.4)
      (`GameplayStatics.PlaySound2D` "/Game/Blueprint/Characters/Character/Enemy/SkeletonEnemy/SkeletonHit.SkeletonHit" 1.0 1.0 0.0 null null))))

(event `/Game/Blueprint/Characters/Character/Enemy/CombatInterface.Dead`
  (set `self.TriggerStun` false)
  (if (not (`self.TriggerStun`))
    (`PrimitiveComponent.SetCollisionEnabled` (`self.Mesh`) "NoCollision")
    (`PrimitiveComponent.SetCollisionEnabled` (`self.enemy_Sword_Mesh`) "NoCollision")
    (`PrimitiveComponent.SetCollisionEnabled` (`self.CapsuleComponent`) "NoCollision")
    (`|PlayMontage` (`self.Mesh`) "/Game/CityofBrass_Enemies/Meshes/Enemy/Charger/Animation/Skeleton_Dead.Skeleton_Dead" 1.75
      (:`then`
        (`GameplayStatics.PlaySound2D` "/Game/Blueprint/Characters/Character/Enemy/SkeletonEnemy/SkeletonDeathCue.SkeletonDeathCue" 1.0 1.0 0.0 null null)
        (`KismetSystemLibrary.Delay` 1.0)
        (`ActorComponent.Activate` (`self.DeathParticle`) false)
        (`GameplayStatics.PlaySound2D` "/Game/Blueprint/Characters/Character/Enemy/DeathParticleCue.DeathParticleCue" 1.0 1.0 0.0 null null)
        (`KismetSystemLibrary.Delay` 0.4)
        (`self.K2_DestroyActor`)))))

(event `self.Sword Collider.OnComponentBeginOverlap`
  (params (OverlappedComponent :type "PrimitiveComponent Object Reference") (OtherActor :type "Actor Object Reference") (OtherComp :type "PrimitiveComponent Object Reference") (OtherBodyIndex :type Integer) (bFromSweep :type Boolean) (SweepResult :type "HitResult Structure (by ref)"))
  (`self.HitPlayer` OtherActor))

(event `self.HitEnemy`
  (params (PlayerDamage :type "Float (double-precision)"))
  (`self.HItEnemyCalculation` PlayerDamage)
  (set `self.StunCounter` (+ (`self.StunCounter`) 1))
  (if (`self.TriggerStun`)
    (if (== (`self.StunCounter`) 3)
      (`|PlayMontage` (`self.Mesh`) "/Game/CityofBrass_Enemies/Meshes/Enemy/Corpse/animation/SkeletonStunned.SkeletonStunned" 2.0
        (:`then`
          (`CharacterMovementComponent.DisableMovement` (`self.CharacterMovement`))
          (set `self.StunCounter` 0)
          (if (not (<= (`/Game/Blueprint/Characters/Character/BP_Status.Health` (`self.Statuss`)) 0.0))
            (`GameplayStatics.PlaySound2D` "/Game/Blueprint/Characters/Character/Enemy/SkeletonEnemy/SkeletonGetHitCue.SkeletonGetHitCue" 1.0 1.0 0.0 null null)
            (`ActorComponent.Activate` (`self.Niagara`) false)
            (`KismetSystemLibrary.Delay` 1.0)
            (`CharacterMovementComponent.SetMovementMode` (`self.CharacterMovement`) "MOVE_Walking" 0)
            (`ActorComponent.Deactivate` (`self.Niagara`))))))))

(fn `UserConstructionScript`
  (`parent.UserConstructionScript`))