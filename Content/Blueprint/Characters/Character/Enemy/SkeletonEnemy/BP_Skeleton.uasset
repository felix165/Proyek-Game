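; BP_Skeleton is a skeleton enemy character that attacks with a sword and removes itself after death.
; MeleeAttack plays a fast attack montage, and overlaps on the SwordCollider pass the other actor to HitPlayer.
; Dead starts the death montage, then destroys the actor after a fixed delay rather than waiting for the montage to finish.
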(event `/Game/Blueprint/Characters/Character/Enemy/CombatInterface.MeleeAttack`
  (`|PlayMontage` (`self.Mesh`) "/Game/CityofBrass_Enemies/Meshes/Enemy/Corpse/animation/Skeleton1AttackFast.Skeleton1AttackFast"))

(event `/Game/Blueprint/Characters/Character/Enemy/CombatInterface.Dead`
  (`|PlayMontage` (`self.Mesh`) "/Game/CityofBrass_Enemies/Meshes/Enemy/Charger/Animation/Skeleton_Dead.Skeleton_Dead"
    (:`then`
      (`KismetSystemLibrary.Delay` 2.5)
      (`self.K2_DestroyActor`))))

(event `self.Sword Collider.OnComponentBeginOverlap`
  (params (OverlappedComponent :type "PrimitiveComponent Object Reference") (OtherActor :type "Actor Object Reference") (OtherComp :type "PrimitiveComponent Object Reference") (OtherBodyIndex :type Integer) (bFromSweep :type Boolean) (SweepResult :type "HitResult Structure (by ref)"))
  (`self.HitPlayer` OtherActor))

(fn `UserConstructionScript`
  (`parent.UserConstructionScript`))