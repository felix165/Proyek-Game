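; Dragon enemy character that sets its own health and defense stats and plays dragon-specific attack and death animations.
; BeginPlay runs the parent setup, then fills in the Statuss values, starting Health at MaxHealth.
; MeleeAttack randomly plays a left or right claw montage.
; Dead starts the death montage and destroys the actor after a short fixed delay.
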(event `self.ReceiveBeginPlay`
  (bind _statuss (`self.Statuss`))
  (`parent.ReceiveBeginPlay`)
  (`|ExecutionSequence`
    (:`then_0`
      (bind _output_get (set `/Game/Blueprint/Characters/Character/BP_Status.MaxHealth` 5000.0 _statuss))
      (set `/Game/Blueprint/Characters/Character/BP_Status.Health` _output_get _statuss))
    (:`then_1`
      (set `/Game/Blueprint/Characters/Character/BP_Status.Defense` 50.0 _statuss))))

(event `/Game/Blueprint/Characters/Character/Enemy/CombatInterface.MeleeAttack`
  (if (== (`KismetMathLibrary.RandomInteger` 2) 1)
    (`|PlayMontage` (`self.Mesh`) "/Game/QuadrapedCreatures/MountainDragon/Animations/AM_DragonLeftClawHit.AM_DragonLeftClawHit")
    (else
      (`|PlayMontage` (`self.Mesh`) "/Game/QuadrapedCreatures/MountainDragon/Animations/AM_DragonRightClawHit.AM_DragonRightClawHit"))))

(event `/Game/Blueprint/Characters/Character/Enemy/CombatInterface.Dead`
  (`|PlayMontage` (`self.Mesh`) "/Game/QuadrapedCreatures/MountainDragon/Animations/AM_DragonDeath.AM_DragonDeath"
    (:`then`
      (`KismetSystemLibrary.Delay` 2.5)
      (`self.K2_DestroyActor`))))

(fn `UserConstructionScript`
  (`parent.UserConstructionScript`))