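; Puzzle stone actor for a three-stone, lights-out style puzzle, where stepping on a stone toggles it and its neighbours.
; On any actor overlap it finds which Puzzle1 stone the player overlaps and flips entries in its Lighted array, with delays and debug prints.
; Most paths then loop over Puzzle1 to set this actor's Box materials from each stone's Lighted state, though both branches assign BasicAsset01.
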(event `self.ReceiveActorBeginOverlap`
  (params (OtherActor :type "Actor Object Reference"))
  (bind _returnvalue (`GameplayStatics.GetPlayerCharacter` 0))
  (bind _lighted (`self.lighted`))
  (bind _lighted_2 (`self.lighted`))
  (bind _lighted_3 (`self.lighted`))
  (bind _puzzle1 (`self.puzzle1`))
  (if (`PrimitiveComponent.IsOverlappingActor` (`/Game/Blueprint/BP_stone1.Box` (`|GetArrayItem` _puzzle1)) _returnvalue)
    (`KismetSystemLibrary.Delay` 1.0)
    (`KismetSystemLibrary.PrintString` "stone 1 over true")
    (if (`|GetArrayItem` _lighted_2)
      (`KismetSystemLibrary.PrintString` "stone 1 light true" true true (struct :`R` 1.0 :`B` 0.169058 :`A` 1.0))
      (`KismetArrayLibrary.Array_Set` _lighted_2)
      (`KismetSystemLibrary.Delay` 1.0)
      (else
        (`KismetSystemLibrary.PrintString` "stone 1 light false" true true (struct :`R` 1.0 :`B` 0.334285 :`A` 1.0))
        (`KismetArrayLibrary.Array_Set` _lighted_2 0 true)
        (`KismetSystemLibrary.Delay` 1.0)))
    (if (`|GetArrayItem` _lighted_2 1)
      (`KismetSystemLibrary.PrintString` " stone 2 light true" true true (struct :`R` 0.019608 :`G` 1.0 :`A` 1.0))
      (`KismetArrayLibrary.Array_Set` _lighted_2 1)
      (`KismetSystemLibrary.Delay` 0.2)
      (else
        (`KismetSystemLibrary.PrintString` " stone 2 light false" true true (struct :`R` 0.019608 :`G` 1.0 :`A` 1.0))
        (`KismetArrayLibrary.Array_Set` _lighted_2 1 true)
        (`KismetSystemLibrary.Delay` 0.2)))
    (for (_array_element _array_index) (`self.puzzle1`) :!label _label
      (if (`|GetArrayItem` (`/Game/Blueprint/BP_stone1.lighted` _array_element) _array_index)
        (`KismetSystemLibrary.PrintString` "set material true" true true (struct :`R` 1.0 :`G` 0.403922 :`A` 1.0))
        (`PrimitiveComponent.SetMaterial` (`self.Box`) _array_index "/Engine/MapTemplates/Materials/BasicAsset01.BasicAsset01")
        (else
          (`KismetSystemLibrary.PrintString` "set material false" true true (struct :`R` 1.0 :`G` 0.403922 :`A` 1.0))
          (`PrimitiveComponent.SetMaterial` (`self.Box`) _array_index "/Engine/MapTemplates/Materials/BasicAsset01.BasicAsset01"))))
    (else
      (`KismetSystemLibrary.Delay` 1.0)
      (`KismetSystemLibrary.PrintString` "stone 1 over false")
      (if (`PrimitiveComponent.IsOverlappingActor` (`/Game/Blueprint/BP_stone1.Box` (`|GetArrayItem` _puzzle1 1)) _returnvalue)
        (if (`|GetArrayItem` _lighted_3 1)
          (`KismetArrayLibrary.Array_Set` _lighted_3 1)
          (else
            (`KismetArrayLibrary.Array_Set` _lighted_3 1 true)))
        (if (`|GetArrayItem` _lighted_3)
          (`KismetArrayLibrary.Array_Set` _lighted_3)
          (if (`|GetArrayItem` _lighted_3 2)
            (`KismetArrayLibrary.Array_Set` _lighted_3 2)
            (goto _label)
            (else
              (`KismetArrayLibrary.Array_Set` _lighted_3 2 true)
              (goto _label)))
          (else
            (`KismetArrayLibrary.Array_Set` _lighted_3 0 true)))
        (elif (`PrimitiveComponent.IsOverlappingActor` (`/Game/Blueprint/BP_stone1.Box` (`|GetArrayItem` _puzzle1 2)) _returnvalue)
          (if (`|GetArrayItem` _lighted 2)
            (`KismetArrayLibrary.Array_Set` _lighted 2)
            (else
              (`KismetArrayLibrary.Array_Set` _lighted 2 true)))
          (if (`|GetArrayItem` _lighted 1)
            (`KismetArrayLibrary.Array_Set` _lighted 1)
            (goto _label)
            (else
              (`KismetArrayLibrary.Array_Set` _lighted 1 true)
              (goto _label))))))))

(fn `UserConstructionScript`)