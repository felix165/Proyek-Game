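; BP_LockedActorRender is the interactive lock actor for a lockpicking minigame, spawned with a widget, target position and locker component.
; Input slides Device0 along a clamped Y range, and its closeness to the target sets how far Device1 may rotate.
; Turning past the threshold reports success to the locker component and destroys the actor, while cancelling reports failure.
; PickBack eases Device1 back to the saved Device0 start rotation via timeline.
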(event `self.ReceiveBeginPlay`
  (set `self.RememberStartRotation` (`SceneComponent.RelativeRotation` (`self.Device_0`))))

(event `Initialize`
  (params (Widget :type "/Game/AdvWorldInteraction/UI/Widgets/Lockpick/WB_Lockpicking Object Reference") (NeededLocation :type "Float (double-precision)") (LockerComp :type "/Game/AdvWorldInteraction/Blueprints/Lock/AC_LockedActor Object Reference"))
  (set `self.Widget` Widget)
  (set `self.NeededLocation` NeededLocation)
  (set `self.LockerComp` LockerComp))

(event `MoveEvent`
  (params (Value :type "Vector2D Structure"))
  (bind (_relativelocation_x _relativelocation_y _relativelocation_z) (`KismetMathLibrary.BreakVector` (`SceneComponent.RelativeLocation` (`self.Device_0`))))
  (`SceneComponent.K2_SetRelativeLocation` (`self.Device_0`) (`KismetMathLibrary.MakeVector` _relativelocation_x (`KismetMathLibrary.FClamp` (+ _relativelocation_y (/ Value_Y 5.0)) -80.0 -40.0) _relativelocation_z) false false))

(event `StopUnlocking`
  (`/Game/AdvWorldInteraction/Blueprints/Lock/AC_LockedActor.EndUnlock` (`self.LockerComp`) false)
  (`SceneComponent.K2_SetRelativeRotation` (`self.Device_1`) (`self.RememberStartRotation`) false false)
  (`self.K2_DestroyActor`))

(event `TryToRotate`
  (bind _device_1 (`self.Device_1`))
  (bind _returnvalue (+ (.pitch (`SceneComponent.RelativeRotation` (`self.Device_1`))) -1.0))
  (`self.CalculateMaxRotation`)
  (`TimelineComponent.Stop` (`self.LerpBack`))
  (if (>= _returnvalue (`self.DynamicStop`))
    (`SceneComponent.K2_SetRelativeRotation` _device_1 (`KismetMathLibrary.MakeRotator` (.roll (`SceneComponent.RelativeRotation` (`self.Device_1`))) _returnvalue (.yaw (`SceneComponent.RelativeRotation` (`self.Device_1`)))) false false)
    (if (<= (.pitch (`SceneComponent.RelativeRotation` _device_1)) -80.0)
      (`/Game/AdvWorldInteraction/Blueprints/Lock/AC_LockedActor.EndUnlock` (`self.LockerComp`) true)
      (`SceneComponent.K2_SetRelativeRotation` (`self.Device_1`) (`self.RememberStartRotation`) false false)
      (`self.K2_DestroyActor`))))

(event `CalculateMaxRotation`
  (set `self.DynamicStop` (`self.CalculateNewDynamicRotation`)))

(event `PickBack`
  (bind (_rememberdynamicrotation_roll _rememberdynamicrotation_pitch) (`KismetMathLibrary.BreakRotator` (`self.RememberDynamicRotation`)))
  (bind _rememberstartrotation (`self.RememberStartRotation`))
  (set `self.RememberDynamicRotation` (`SceneComponent.RelativeRotation` (`self.Device_1`)))
  (bind (_direction _alpha) (`Timeline|LerpBack` :!via `PlayFromStart`)
    (:`Update`
      (`SceneComponent.K2_SetRelativeRotation` (`self.Device_1`) (`KismetMathLibrary.RLerp` (`KismetMathLibrary.MakeRotator` (.roll _rememberstartrotation) _rememberdynamicrotation_pitch (.yaw _rememberstartrotation)) _rememberstartrotation _alpha) false false))))

(fn `CalculateNewDynamicRotation`
  (returns (ReturnValue :type "Float (double-precision)"))
  (bind (_relativelocation_x _relativelocation_y) (`KismetMathLibrary.BreakVector` (`SceneComponent.RelativeLocation` (`self.Device_0`))))
  (return (* (`KismetMathLibrary.Abs` (- 90.0 (* (`KismetMathLibrary.Abs` (- 1.0 (/ (`KismetMathLibrary.Abs` (`self.NeededLocation`)) (`KismetMathLibrary.Abs` _relativelocation_y)))) 100.0))) -1.0)))

(fn `UserConstructionScript`)