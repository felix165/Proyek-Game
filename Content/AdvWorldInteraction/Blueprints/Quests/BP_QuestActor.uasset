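; World quest point actor with a widget marker and an overlap sphere for completing overlap-type tasks.
; Tick loops over all Characters, setting widget visibility from the render-distance setting, with markered quests always shown.
; Sphere overlap by a Character with AC_QuestsHandler takes ownership and completes matching task types through that component.
; ChangeState, run shortly after BeginPlay, rebuilds marked-area info as tracked or untracked from the widget's Markered flag.
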(event `self.ReceiveBeginPlay`
  (`KismetSystemLibrary.Delay` 0.5)
  (`self.ChangeState`))

(event `ChangeState`
  (set `self.AreaInfo` (`self.GetUpdatedMarkedAreaInfo`)))

(event `self.ReceiveTick`
  (params (DeltaSeconds :type "Float (single-precision)"))
  (bind _outactors (`GameplayStatics.GetAllActorsOfClass` "/Script/Engine.Character"))
  (for _array_element _outactors
    (if (<= (`KismetMathLibrary.VSize` (- (`self.K2_GetActorLocation` _array_element) (`self.K2_GetActorLocation`))) (`.RenderWorldWidget_48_3935E7F64E206F58FE8FEB8931EC1C57` (break `/Game/AdvWorldInteraction/Blueprints/GameSettings/S_GameSettings` (`/Game/AdvWorldInteraction/Blueprints/Other/BPL_DataTableSlotInfo.GetGameSettingsInfo` (`self.GameSettings`)))))
      (`SceneComponent.SetVisibility` (`self.Widget`) true false :!label _label)
      (elif (`/Game/AdvWorldInteraction/UI/Widgets/WorldMap/Quest/WB_QuestPoint.Markered` (`self.GetQuestWidget`))
        (goto _label)
        (else
          (`SceneComponent.SetVisibility` (`self.Widget`) false false))))))

(event `self.Sphere.OnComponentBeginOverlap`
  (params (OverlappedComponent :type "PrimitiveComponent Object Reference") (OtherActor :type "Actor Object Reference") (OtherComp :type "PrimitiveComponent Object Reference") (OtherBodyIndex :type Integer) (bFromSweep :type Boolean) (SweepResult :type "HitResult Structure (by ref)"))
  (bind _task (`self.Task`))
  ;[1 1 1] Multiplayered Overlap
  (bind _ascharacter (cast `Character` OtherActor))
  (bind _returnvalue (`self.GetComponentByClass` _ascharacter "/Game/AdvWorldInteraction/Blueprints/MapComponents/AC_QuestsHandler.AC_QuestsHandler_C"))
  (`/Engine/EditorBlueprintResources/StandardMacros.IsValid` _returnvalue
    (:`Is Valid`
      (`self.SetOwner` _ascharacter)
      (if (`|EnumEquality` (`.Type_11_081F2ED04F4ACF3322646AB069CFE0CF` (break `/Game/AdvWorldInteraction/Blueprints/Information/Tasks/S_PlaceTaskList` (`/Game/AdvWorldInteraction/Blueprints/Other/BPL_DataTableSlotInfo.GetTaskInfo` (`.Task_18_67F2EAB0420DE50E7CBF92962B93578C` (break `/Game/AdvWorldInteraction/Blueprints/Information/Tasks/S_pTaskListInv` _task))))) "NewEnumerator3")
        (`/Game/AdvWorldInteraction/Blueprints/MapComponents/AC_QuestsHandler.CompleteTaskType` _returnvalue _task self)))))

(fn `GetQuestWidget`
  (returns (`AsWB Quest Point` :type "/Game/AdvWorldInteraction/UI/Widgets/WorldMap/Quest/WB_QuestPoint Object Reference"))
  (bind _aswb_quest_point (cast `/Game/AdvWorldInteraction/UI/Widgets/WorldMap/Quest/WB_QuestPoint` (`WidgetComponent.GetUserWidgetObject` (`self.Widget`))))
  (return _aswb_quest_point))

(fn `GetUpdatedMarkedAreaInfo`
  (returns (S_AreaState :type "/Game/AdvWorldInteraction/Blueprints/Information/Area/S_AreaState Structure"))
  (return (make `/Game/AdvWorldInteraction/Blueprints/Information/Area/S_AreaState` (select `bool` (`/Game/AdvWorldInteraction/UI/Widgets/WorldMap/Quest/WB_QuestPoint.Markered` (`self.GetQuestWidget`)) :`false` (`self.UntrackedTaskInfo`) :`true` (`self.TrackedTaskInfo`)) true (`|MakeArray` (struct) :!type "/Game/AdvWorldInteraction/Blueprints/Information/Tasks/S_pTaskListInv Structure") (`|MakeArray` (struct) :!type "/Game/AdvWorldInteraction/Blueprints/Information/Tasks/S_pTaskListInv Structure") (`|MakeArray` (struct) :!type "/Game/AdvWorldInteraction/Blueprints/Information/Items/S_Reward Structure"))))

(fn `TryToCompleteOverlapTask`
  (params (QuestH :type "/Game/AdvWorldInteraction/Blueprints/MapComponents/AC_QuestsHandler Object Reference"))
  (bind _quests (`/Game/AdvWorldInteraction/Blueprints/MapComponents/AC_QuestsHandler.Quests` QuestH))
  (bind _task (`self.Task`))
  (if (`KismetArrayLibrary.Array_Contains` _quests _task)
    (if (`|EnumEquality` (`.Type_11_081F2ED04F4ACF3322646AB069CFE0CF` (break `/Game/AdvWorldInteraction/Blueprints/Information/Tasks/S_PlaceTaskList` (`/Game/AdvWorldInteraction/Blueprints/Other/BPL_DataTableSlotInfo.GetTaskInfo` (`.Task_18_67F2EAB0420DE50E7CBF92962B93578C` (break `/Game/AdvWorldInteraction/Blueprints/Information/Tasks/S_pTaskListInv` _task))))) "NewEnumerator3")
      (`/Game/AdvWorldInteraction/Blueprints/MapComponents/AC_QuestsHandler.OnTaskCompleted` QuestH (`KismetArrayLibrary.Array_Find` _quests _task))
      (`self.SetLifeSpan` 0.2))))

(fn `UserConstructionScript`
  (`parent.UserConstructionScript`))