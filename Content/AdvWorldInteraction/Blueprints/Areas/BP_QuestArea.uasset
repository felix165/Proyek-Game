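; Quest area Blueprint that tracks whether its quest objective is completed.
; QuestUpdate switches on QuestType; its Defeat Enemy case recounts the EnemiesToDefeat with zero Health and sets Completed once the count matches the list length.
; The event graph and construction script are empty, so the check runs only when QuestUpdate is called.
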(fn `QuestUpdate`
  (switch `/Game/Blueprint/Information/Enum_QuestType` (`self.QuestType`)
    (:`NewEnumerator0`
      (bind _output_get (set `self.Enemies_Counter` 0))
      (for _array_element (`self.EnemiesToDefeat`)
        (if (== (`/Game/Blueprint/Characters/Character/BP_Status.Health` (`/Game/Blueprint/Characters/Character/Enemy/BP_EnemiesBase.Statuss` _array_element)) 0.0)
          (bind _result (`/Engine/EditorBlueprintResources/StandardMacros.IncrementInt` _output_get)
            (:`  `
              (if (== _result (`KismetArrayLibrary.Array_Length` (`self.EnemiesToDefeat`)))
                (set `self.Completed` true)))))))))

(fn `UserConstructionScript`)