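; AC_Minimap is an actor component that gives its owning actor a minimap handler.
; On BeginPlay it calls a server-named event that spawns a BP_MinimapHandler actor and passes it to an owning-client-named event.
; That second event stores the reference and, if valid, sets the handler's owner to the component's owner and attaches it there with relative transform rules.
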(event `self.ReceiveBeginPlay`
  ;[1 1 1] Spawn Map Helper
  (`self.SpawnActor -Server`))

(event `SpawnActor -OC`
  (params (Target :type "/Game/AdvWorldInteraction/Blueprints/MapComponents/Minimap/BP_MinimapHandler Object Reference"))
  (bind _returnvalue (`self.GetOwner`))
  ;[1 1 1] Spawn Map Helper
  (bind _output_get (set `self.SpawnedActor` Target))
  (`/Engine/EditorBlueprintResources/StandardMacros.IsValid` _output_get
    (:`Is Valid`
      (`Actor.SetOwner` (`self.SpawnedActor`) _returnvalue)
      (`Actor.K2_AttachToActor` (`self.SpawnedActor`) _returnvalue "None" "KeepRelative" "KeepRelative" "KeepRelative" true))))

(event `SpawnActor -Server`
  ;[1 1 1] Spawn Map Helper
  (bind _returnvalue (`|SpawnActorFromClass` "/Game/AdvWorldInteraction/Blueprints/MapComponents/Minimap/BP_MinimapHandler.BP_MinimapHandler_C" (`KismetMathLibrary.MakeTransform` (0.0 0.0 0.0)) "Undefined" "OverrideRootScale" null null))
  (`self.SpawnActor -OC` _returnvalue))