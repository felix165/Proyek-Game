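; Player character component that holds the quest list and current quest, handling task markers, completion and saving.
; ShowTask spawns a world-map marker at the quest's first actor.
; Completing an Item or Overlap task removes it, refreshes map, compass and quest UI, grants the quest giver's money, XP and items, and expires the target.
; SaveQuests stores quests, quest-giver data and marker actors in a save slot; BeginPlay restores them, respawning the markers.
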(event `self.ReceiveBeginPlay`
  ;[1 1 1] Initialize Owner as Character Class
  (bind _ascharacter (cast `Character` (`self.GetOwner`)))
  (set `self.Player` _ascharacter)
  (`self.LoadQuests`))

(event `ShowTask`
  (params (Index :type Integer))
  (bind _output (`|GetArrayItem` (`.Actors_17_34CA0055473DFF6A2F79C9B31B76545E` (break `/Game/AdvWorldInteraction/Blueprints/Information/Tasks/S_pTaskListInv` (`|GetArrayItem` (`self.Quests`) Index)))))
  ;[1 1 1] Add a new task to the player and the map
  (set `self.CurrentQuestIndex` Index)
  (`/Engine/EditorBlueprintResources/StandardMacros.IsValid` _output
    (:`Is Valid`
      (`/Game/AdvWorldInteraction/Blueprints/MapComponents/WorldMap/AC_WorldMap.SpawnQuestionBP` (`Actor.GetComponentByClass` (`self.Player`) "/Game/AdvWorldInteraction/Blueprints/MapComponents/WorldMap/AC_WorldMap.AC_WorldMap_C") (`Actor.K2_GetActorLocation` _output) (`self.Player`) "/Game/AdvWorldInteraction/UI/Textures/Tasks/Quests/T_QuestPlace.T_QuestPlace" (`self.GetCurrentQuest`)))))

(event `OnTaskCompleted`
  (params (Index :type Integer))
  ;[1 1 1] Task is completed Event
  (`KismetSystemLibrary.Delay` 0.1)
  (`KismetArrayLibrary.Array_Remove` (`self.Quests`) Index)
  (`self.RecreateMapAndCompass`)
  (set `self.CurrentQuestIndex` -1)
  (`/Game/AdvWorldInteraction/UI/Widgets/Quests/WB_Quests.Update` (`/Game/AdvWorldInteraction/UI/Widgets/Menu/WB_MainGUI.WB_Quests` (`/Game/AdvWorldInteraction/Blueprints/WidgetHandler/AC_MainWidgetHandler.WB_MainGUI` (`Actor.GetComponentByClass` (`self.Player`) "/Game/AdvWorldInteraction/Blueprints/WidgetHandler/AC_MainWidgetHandler.AC_MainWidgetHandler_C")))))

(fn `CompleteTaskType`
  (params (Task :type "/Game/AdvWorldInteraction/Blueprints/Information/Tasks/S_pTaskListInv Structure (by ref)") (Target :type "Actor Object Reference"))
  (locals (l_CurrentTask :type "/Game/AdvWorldInteraction/Blueprints/Information/Tasks/S_pTaskListInv Structure"))
  (bind _quests (`self.Quests`))
  (bind _l_currenttask (`local.l_CurrentTask`))
  ;[1 1 1] Try to find the task and complete it on success
  (set `local.l_CurrentTask` Task)
  (if (`KismetArrayLibrary.Array_Contains` _quests _l_currenttask)
    (switch `/Game/AdvWorldInteraction/Blueprints/Information/Tasks/E_TaskType` (`.Type_11_081F2ED04F4ACF3322646AB069CFE0CF` (break `/Game/AdvWorldInteraction/Blueprints/Information/Tasks/S_PlaceTaskList` (`/Game/AdvWorldInteraction/Blueprints/Other/BPL_DataTableSlotInfo.GetTaskInfo` (`.Task_18_67F2EAB0420DE50E7CBF92962B93578C` (break `/Game/AdvWorldInteraction/Blueprints/Information/Tasks/S_pTaskListInv` _l_currenttask)))))
      (:`NewEnumerator2`
        _)
      (:`NewEnumerator3`
        _))
    (`self.OnTaskCompleted` (`KismetArrayLibrary.Array_Find` _quests (`local.l_CurrentTask`)))
    (bind _asbp_quest_character (cast `/Game/AdvWorldInteraction/Blueprints/Quests/BP_QuestCharacter` (`.QuestOrderPerson_21_6BEE75064AF0CEDDD605AC9185807C73` (break `/Game/AdvWorldInteraction/Blueprints/Information/Tasks/S_pTaskListInv` (`local.l_CurrentTask`))))
      (:`then`
        (`self.GiveQuestRewardToPLayer` (`/Game/AdvWorldInteraction/Blueprints/Quests/BP_QuestCharacter.Reward` _asbp_quest_character) (`self.Player`)))
      (:`CastFailed`
        _))
    (`Actor.SetLifeSpan` Target 0.05)))

(fn `GetCurrentQuest`
  (returns (CurrentQuest :type "/Game/AdvWorldInteraction/Blueprints/Information/Tasks/S_pTaskListInv Structure"))
  (return (`|GetArrayItem` (`self.Quests`) (`self.CurrentQuestIndex`))))

(fn `GiveQuestRewardToPLayer`
  (params (Reward :type "Array of /Game/AdvWorldInteraction/Blueprints/Information/Items/S_Reward Structure") (Target :type "Actor Object Reference"))
  (bind (_money _exp _items) (`/Game/AdvWorldInteraction/Blueprints/Other/BPL_DataTableSlotInfo.SplitRewardArray` Reward))
  (`/Game/AdvWorldInteraction/Blueprints/Other/BPL_DataTableSlotInfo.AddMoneyToActor` Target _money)
  (`/Game/AdvWorldInteraction/Blueprints/Other/BPL_DataTableSlotInfo.AddExpToActor` Target _exp)
  (`/Game/AdvWorldInteraction/Blueprints/Other/BPL_DataTableSlotInfo.AddItemsToActor` Target _items)
  (bind _returnvalue (`|CreateWidget` "/Game/AdvWorldInteraction/UI/Widgets/AnnounceScreen/WB_RewardAnnouncment.WB_RewardAnnouncment_C" null _money _exp _items false true))
  (`UserWidget.AddToViewport` _returnvalue 0))

(fn `LoadQuests`
  (bind _player (`self.Player`))
  (bind _returnvalue (`GameplayStatics.DoesSaveGameExist` (`self.QuestSlot`)))
  (if _returnvalue
    (bind _returnvalue_2 (`GameplayStatics.LoadGameFromSlot` (`self.QuestSlot`)))
    (bind _assave_quests (cast `/Game/AdvWorldInteraction/Blueprints/MapComponents/ComponentsSaves/Quests/Save_Quests` _returnvalue_2))
    (set `self.Quests` (`/Game/AdvWorldInteraction/Blueprints/MapComponents/ComponentsSaves/Quests/Save_Quests.sQuests` _assave_quests))
    (set `self.CurrentQuestIndex` (`/Game/AdvWorldInteraction/Blueprints/MapComponents/ComponentsSaves/Quests/Save_Quests.sCurrentQuest` _assave_quests))
    (bind _outactors (`GameplayStatics.GetAllActorsOfClass` "/Game/AdvWorldInteraction/Blueprints/Quests/BP_QuestCharacter.BP_QuestCharacter_C"))
    (for _array_element _outactors
      (for _array_element_2 (`/Game/AdvWorldInteraction/Blueprints/MapComponents/ComponentsSaves/Quests/Save_Quests.sCharacters` _assave_quests)
        (bind (_reference _task _reward) (break `/Game/AdvWorldInteraction/Blueprints/MapComponents/ComponentsSaves/Quests/S_SaveQuestCharacter` _array_element_2))
        (if (== _array_element _reference)
          (set `/Game/AdvWorldInteraction/Blueprints/Quests/BP_QuestCharacter.Task` _task _array_element)
          (set `/Game/AdvWorldInteraction/Blueprints/Quests/BP_QuestCharacter.Reward` _reward _array_element))))
    (for _array_element_3 (`/Game/AdvWorldInteraction/Blueprints/MapComponents/ComponentsSaves/Quests/Save_Quests.sActors` _assave_quests)
      (bind (_location _task_2 _markered_) (break `/Game/AdvWorldInteraction/Blueprints/MapComponents/ComponentsSaves/Quests/S_SaveQuestActor` _array_element_3))
      (bind _returnvalue_3 (`|SpawnActorFromClass` "/Game/AdvWorldInteraction/Blueprints/Quests/BP_QuestActor.BP_QuestActor_C" (`KismetMathLibrary.Conv_VectorToTransform` _location) "Undefined" "OverrideRootScale" null null))
      (set `/Game/AdvWorldInteraction/Blueprints/Quests/BP_QuestActor.Task` _task_2 _returnvalue_3)
      (bind _aswb_quest_point (`/Game/AdvWorldInteraction/Blueprints/Quests/BP_QuestActor.GetQuestWidget` _returnvalue_3))
      (bind _output_get (set `/Game/AdvWorldInteraction/UI/Widgets/WorldMap/Quest/WB_QuestPoint.Markered` _markered_ _aswb_quest_point))
      (set `/Game/AdvWorldInteraction/Blueprints/Areas/BP_NavPoint.Marker?` _output_get _returnvalue_3)
      (set `/Game/AdvWorldInteraction/UI/Widgets/WorldMap/Quest/WB_QuestPoint.MapRef` (`Actor.GetComponentByClass` _player "/Game/AdvWorldInteraction/Blueprints/MapComponents/WorldMap/AC_WorldMap.AC_WorldMap_C") _aswb_quest_point)
      (set `/Game/AdvWorldInteraction/UI/Widgets/WorldMap/Quest/WB_QuestPoint.Player` _player _aswb_quest_point)
      (set `/Game/AdvWorldInteraction/UI/Widgets/WorldMap/Quest/WB_QuestPoint.Location` (`Actor.K2_GetActorLocation` _returnvalue_3) _aswb_quest_point))))

(fn `MakeSaveActorsVariable`
  (params (TargetArray :type "Array of /Game/AdvWorldInteraction/Blueprints/MapComponents/ComponentsSaves/Quests/S_SaveQuestActor Structure (by ref)"))
  (bind _outactors (`GameplayStatics.GetAllActorsOfClass` "/Game/AdvWorldInteraction/Blueprints/Quests/BP_QuestActor.BP_QuestActor_C"))
  (for _array_element _outactors
    (`KismetArrayLibrary.Array_Add` TargetArray (make `/Game/AdvWorldInteraction/Blueprints/MapComponents/ComponentsSaves/Quests/S_SaveQuestActor` (`Actor.K2_GetActorLocation` _array_element) (`/Game/AdvWorldInteraction/Blueprints/Quests/BP_QuestActor.Task` _array_element) (`/Game/AdvWorldInteraction/UI/Widgets/WorldMap/Quest/WB_QuestPoint.Markered` (`/Game/AdvWorldInteraction/Blueprints/Quests/BP_QuestActor.GetQuestWidget` _array_element))))))

(fn `MakeSaveCharactersVariable`
  (params (TargetArray :type "Array of /Game/AdvWorldInteraction/Blueprints/MapComponents/ComponentsSaves/Quests/S_SaveQuestCharacter Structure (by ref)"))
  (bind _outactors (`GameplayStatics.GetAllActorsOfClass` "/Game/AdvWorldInteraction/Blueprints/Quests/BP_QuestCharacter.BP_QuestCharacter_C"))
  (for _array_element _outactors
    (`KismetArrayLibrary.Array_Add` TargetArray (make `/Game/AdvWorldInteraction/Blueprints/MapComponents/ComponentsSaves/Quests/S_SaveQuestCharacter` _array_element (`/Game/AdvWorldInteraction/Blueprints/Quests/BP_QuestCharacter.GetTask` _array_element) (`/Game/AdvWorldInteraction/Blueprints/Quests/BP_QuestCharacter.Reward` _array_element)))))

(fn `RecreateMapAndCompass`
  (bind _player (`self.Player`))
  (bind _wb_compass (`/Game/AdvWorldInteraction/Blueprints/Other/BPL_DataTableSlotInfo.GetCharacterCompass` _player))
  ;[1 1 1] Remove Marker From All Quests
  (bind _outactors (`GameplayStatics.GetAllActorsOfClass` "/Game/AdvWorldInteraction/Blueprints/Quests/BP_QuestActor.BP_QuestActor_C"))
  (for _array_element _outactors
    (set `/Game/AdvWorldInteraction/Blueprints/Areas/BP_NavPoint.Marker?` false _array_element)
    (set `/Game/AdvWorldInteraction/UI/Widgets/WorldMap/Quest/WB_QuestPoint.Markered` false (`/Game/AdvWorldInteraction/Blueprints/Quests/BP_QuestActor.GetQuestWidget` _array_element))
    (`/Game/AdvWorldInteraction/Blueprints/Quests/BP_QuestActor.ChangeState` _array_element))
  ;[1 1 1] Recreate Quests on the Map
  (`/Game/AdvWorldInteraction/Blueprints/MapComponents/WorldMap/AC_WorldMap.AddQuestToTheMap` (`Actor.GetComponentByClass` _player "/Game/AdvWorldInteraction/Blueprints/MapComponents/WorldMap/AC_WorldMap.AC_WorldMap_C"))
  (`/Engine/EditorBlueprintResources/StandardMacros.IsValid` _wb_compass
    (:`Is Valid`
      (`/Game/AdvWorldInteraction/UI/Widgets/Compas/WB_Compass.Recreate` _wb_compass))))

(fn `SaveQuests`
  (locals (SaveGAme :type "/Game/AdvWorldInteraction/Blueprints/MapComponents/ComponentsSaves/Quests/Save_Quests Object Reference") (SaveCharacters :type "Array of /Game/AdvWorldInteraction/Blueprints/MapComponents/ComponentsSaves/Quests/S_SaveQuestCharacter Structure") (SaveActors :type "Array of /Game/AdvWorldInteraction/Blueprints/MapComponents/ComponentsSaves/Quests/S_SaveQuestActor Structure"))
  (bind _savegame (`local.SaveGAme`))
  (bind _returnvalue (`GameplayStatics.DoesSaveGameExist` (`self.QuestSlot`)))
  (if _returnvalue
    (bind _returnvalue_2 (`GameplayStatics.LoadGameFromSlot` (`self.QuestSlot`)))
    (bind _assave_quests (cast `/Game/AdvWorldInteraction/Blueprints/MapComponents/ComponentsSaves/Quests/Save_Quests` _returnvalue_2))
    (set `local.SaveGAme` _assave_quests)
    (else
      (bind _returnvalue_3 (`GameplayStatics.CreateSaveGameObject` "/Game/AdvWorldInteraction/Blueprints/MapComponents/ComponentsSaves/Quests/Save_Quests.Save_Quests_C"))
      (set `local.SaveGAme` _returnvalue_3)))
  (set `/Game/AdvWorldInteraction/Blueprints/MapComponents/ComponentsSaves/Quests/Save_Quests.sQuests` (`self.Quests`) _savegame)
  (set `/Game/AdvWorldInteraction/Blueprints/MapComponents/ComponentsSaves/Quests/Save_Quests.sCurrentQuest` (`self.CurrentQuestIndex`) _savegame)
  (`self.MakeSaveCharactersVariable` (`local.SaveCharacters`))
  (set `/Game/AdvWorldInteraction/Blueprints/MapComponents/ComponentsSaves/Quests/Save_Quests.sCharacters` (`local.SaveCharacters`) (`local.SaveGAme`))
  (`self.MakeSaveActorsVariable` (`local.SaveActors`))
  (set `/Game/AdvWorldInteraction/Blueprints/MapComponents/ComponentsSaves/Quests/Save_Quests.sActors` (`local.SaveActors`) (`local.SaveGAme`))
  (`GameplayStatics.SaveGameToSlot` (`local.SaveGAme`) (`self.QuestSlot`)))

(fn `SetNewQuestSelected`
  (params (ItemToFind :type "/Game/AdvWorldInteraction/Blueprints/Information/Tasks/S_pTaskListInv Structure (by ref)"))
  (bind _quests (`self.Quests`))
  (if (`KismetArrayLibrary.Array_Contains` _quests ItemToFind)
    (set `self.CurrentQuestIndex` (`KismetArrayLibrary.Array_Find` _quests ItemToFind))
    (`/Game/AdvWorldInteraction/UI/Widgets/Quests/WB_Quests.Update` (`/Game/AdvWorldInteraction/UI/Widgets/Menu/WB_MainGUI.WB_Quests` (`/Game/AdvWorldInteraction/Blueprints/WidgetHandler/AC_MainWidgetHandler.WB_MainGUI` (`Actor.GetComponentByClass` (`self.Player`) "/Game/AdvWorldInteraction/Blueprints/WidgetHandler/AC_MainWidgetHandler.AC_MainWidgetHandler_C"))))))