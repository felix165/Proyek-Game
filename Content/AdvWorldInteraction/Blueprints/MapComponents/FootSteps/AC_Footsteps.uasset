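; Footsteps component that plays a surface-dependent step sound at its owner's location whenever LegEvent is called.
; LegEvent line-traces down from the owner on the Visibility channel and reads the hit physical material's surface type, staying silent if there is no material.
; GetSurfceSound scans the rows of StepsDataTable for that type's sound and, if none matches, calls itself recursively with the default surface type.
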(event `LegEvent`
  (bind _returnvalue (`Actor.K2_GetActorLocation` (`self.GetOwner`)))
  ;[1 1 1] Legs Sound Line Trace And Play sound at location
  (bind _outhit (`KismetSystemLibrary.LineTraceSingle` _returnvalue (`KismetMathLibrary.MakeVector` (.x _returnvalue) (.y _returnvalue) -5000.0) "TraceTypeQuery1"))
  (bind (_bblockinghit _binitialoverlap _time _distance _location _impactpoint _normal _impactnormal _physmat) (`GameplayStatics.BreakHitResult` _outhit))
  (`/Engine/EditorBlueprintResources/StandardMacros.IsValid` _physmat
    (:`Is Valid`
      (bind _sound (`self.GetSurfceSound` (`PhysicalMaterial.SurfaceType` _physmat)))
      (`/Engine/EditorBlueprintResources/StandardMacros.IsValid` _sound
        (:`Is Valid`
          (`GameplayStatics.PlaySoundAtLocation` _sound (`Actor.K2_GetActorLocation` (`self.GetOwner`))))))))

(fn `GetSurfceSound`
  (params (SurfaceType :type "EPhysicalSurface Enum" :default "SurfaceType_Default"))
  (returns (Sound :type "SoundCue Object Reference"))
  (bind _outrownames (`DataTableFunctionLibrary.GetDataTableRowNames` (`self.StepsDataTable`)))
  (for _array_element _outrownames
    (bind _returnvalue (`|GetDataTableRow` (`self.StepsDataTable`) _array_element)
      (:`then`
        (bind (_type _sound) (break `/Game/AdvWorldInteraction/Blueprints/Information/FootSteps/S_FootstepType` _returnvalue))
        (if (`|EnumEquality` _type SurfaceType)
          (return _sound)))))
  (return (`self.GetSurfceSound` "SurfaceType_Default")))