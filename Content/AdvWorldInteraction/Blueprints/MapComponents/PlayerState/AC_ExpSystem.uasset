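; Player experience and leveling component that tracks current XP, level and the threshold for the next level.
; AddExp loops through level-ups, carrying surplus XP over and scaling the threshold by a multiplier, then refreshes the XP and money widget through the owner's AC_MainWidgetHandler.
; Progress loads from a Save_Exp slot on BeginPlay, while SaveExp writes it back, creating the save object if none exists.
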(event `self.ReceiveBeginPlay`
  (`self.LoadExp`))

(fn `AddExp`
  (params (Value :type "Float (double-precision)"))
  (bind _output_get (set `self.CurrentExp` (+ Value (`self.CurrentExp`))))
  (if (>= _output_get (`self.ExpToTheNextLevel`)) :!label _label
    (`self.LevelUp`)
    (`/Engine/EditorBlueprintResources/StandardMacros.IncrementInt` (`self.CurrentLevel`)
      (:`  `
        (goto _label)))
    (else
      (`self.UpdateWidget`)
      (return))))

(fn `LevelUp`
  (set `self.CurrentExp` (- (`self.CurrentExp`) (`self.ExpToTheNextLevel`)))
  (set `self.ExpToTheNextLevel` (* (`self.ExpToTheNextLevel`) (`self.NextExpMultiplayer`))))

(fn `LoadExp`
  (bind _returnvalue (`GameplayStatics.DoesSaveGameExist` (`self.ExpSlot`)))
  (if _returnvalue
    (bind _returnvalue_2 (`GameplayStatics.LoadGameFromSlot` (`self.ExpSlot`)))
    (bind _assave_exp (cast `/Game/AdvWorldInteraction/Blueprints/MapComponents/ComponentsSaves/Save_Exp` _returnvalue_2))
    (set `self.CurrentExp` (`/Game/AdvWorldInteraction/Blueprints/MapComponents/ComponentsSaves/Save_Exp.sExp` _assave_exp))
    (set `self.ExpToTheNextLevel` (`/Game/AdvWorldInteraction/Blueprints/MapComponents/ComponentsSaves/Save_Exp.sExpToNextLevel` _assave_exp))
    (set `self.CurrentLevel` (`/Game/AdvWorldInteraction/Blueprints/MapComponents/ComponentsSaves/Save_Exp.sCurrentLevel` _assave_exp))))

(fn `SaveExp`
  (bind _savegame (`self.SaveGAme`))
  (bind _returnvalue (`GameplayStatics.DoesSaveGameExist` (`self.ExpSlot`)))
  (if _returnvalue
    (bind _returnvalue_2 (`GameplayStatics.LoadGameFromSlot` (`self.ExpSlot`)))
    (bind _assave_exp (cast `/Game/AdvWorldInteraction/Blueprints/MapComponents/ComponentsSaves/Save_Exp` _returnvalue_2))
    (set `self.SaveGAme` _assave_exp)
    (else
      (bind _returnvalue_3 (`GameplayStatics.CreateSaveGameObject` "/Game/AdvWorldInteraction/Blueprints/MapComponents/ComponentsSaves/Save_Exp.Save_Exp_C"))
      (set `self.SaveGAme` _returnvalue_3)))
  (set `/Game/AdvWorldInteraction/Blueprints/MapComponents/ComponentsSaves/Save_Exp.sExp` (`self.CurrentExp`) _savegame)
  (set `/Game/AdvWorldInteraction/Blueprints/MapComponents/ComponentsSaves/Save_Exp.sCurrentLevel` (`self.CurrentLevel`) _savegame)
  (set `/Game/AdvWorldInteraction/Blueprints/MapComponents/ComponentsSaves/Save_Exp.sExpToNextLevel` (`self.ExpToTheNextLevel`) _savegame)
  (`GameplayStatics.SaveGameToSlot` (`self.SaveGAme`) (`self.ExpSlot`)))

(fn `UpdateWidget`
  (bind _returnvalue (`Actor.GetComponentByClass` (`self.GetOwner`) "/Game/AdvWorldInteraction/Blueprints/WidgetHandler/AC_MainWidgetHandler.AC_MainWidgetHandler_C"))
  (bind _wb_maingui (`/Game/AdvWorldInteraction/Blueprints/WidgetHandler/AC_MainWidgetHandler.WB_MainGUI` _returnvalue))
  (bind _wb_expandmoney (`/Game/AdvWorldInteraction/UI/Widgets/Menu/WB_MainGUI.WB_ExpAndMoney` _wb_maingui))
  (`/Engine/EditorBlueprintResources/StandardMacros.IsValid` _returnvalue
    (:`Is Valid`
      (`/Engine/EditorBlueprintResources/StandardMacros.IsValid` _wb_maingui
        (:`Is Valid`
          (`/Engine/EditorBlueprintResources/StandardMacros.IsValid` _wb_expandmoney
            (:`Is Valid`
              (`/Game/AdvWorldInteraction/UI/Widgets/Player/WB_ExpAndMoney.UpdateVariables` _wb_expandmoney))))))))