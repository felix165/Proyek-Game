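; Inventory component that holds a player's items and persists them to a save slot.
; It loads the inventory from a Save_Inventory object on BeginPlay, and SaveInventory writes it back, creating the save object if none exists.
; Initialize caches the owning character, its controller and the inventory widget, which AddItems refreshes.
; ToggleInventory shows or hides that widget, switching input mode and mouse cursor to match.
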(event `self.ReceiveBeginPlay`
  (`self.LoadInventory`))

(event `Initialize`
  (params (Widget :type "/Game/AdvWorldInteraction/UI/Widgets/Inventory/WB_Inventory Object Reference"))
  ;[1 1 1] Initialize player
  (set `self.Widget` Widget)
  (bind _ascharacter (cast `Character` (`self.GetOwner`)))
  (bind _output_get (set `self.Player` _ascharacter))
  (bind _asplayer_controller (cast `PlayerController` (`Pawn.GetController` _output_get)))
  (set `self.PlayerController` _asplayer_controller))

(event `ToggleInventory`
  (bind _playercontroller (`self.PlayerController`))
  ;[1 1 1] Toggle inventory logic
  (if (`|EnumEquality` (`Widget.GetVisibility` (`self.Widget`)) "Visible")
    (`Widget.SetVisibility` (`self.Widget`) "Hidden")
    (`WidgetBlueprintLibrary.SetInputMode_GameOnly` _playercontroller)
    (set `PlayerController.bShowMouseCursor` false _playercontroller)
    (else
      (`Widget.SetVisibility` (`self.Widget`) "Visible")
      (`WidgetBlueprintLibrary.SetInputMode_GameAndUIEx` _playercontroller (`self.Widget`))
      (set `PlayerController.bShowMouseCursor` true _playercontroller))))

(fn `AddItems`
  (params (Items :type "Array of DataTableRowHandle Structure"))
  (for _array_element Items
    (`KismetArrayLibrary.Array_Add` (`self.Inventory`) _array_element))
  (`self.UpdateInventory`))

(fn `LoadInventory`
  (bind _returnvalue (`GameplayStatics.DoesSaveGameExist` (`self.InventorySlot`)))
  (if _returnvalue
    (bind _returnvalue_2 (`GameplayStatics.LoadGameFromSlot` (`self.InventorySlot`)))
    (bind _assave_inventory (cast `/Game/AdvWorldInteraction/Blueprints/MapComponents/ComponentsSaves/Save_Inventory` _returnvalue_2))
    (set `self.Inventory` (`/Game/AdvWorldInteraction/Blueprints/MapComponents/ComponentsSaves/Save_Inventory.sInventory` _assave_inventory))))

(fn `SaveInventory`
  (bind _returnvalue (`GameplayStatics.DoesSaveGameExist` (`self.InventorySlot`)))
  (if _returnvalue
    (bind _returnvalue_2 (`GameplayStatics.LoadGameFromSlot` (`self.InventorySlot`)))
    (bind _assave_inventory (cast `/Game/AdvWorldInteraction/Blueprints/MapComponents/ComponentsSaves/Save_Inventory` _returnvalue_2))
    (set `self.SaveGAme` _assave_inventory)
    (else
      (bind _returnvalue_3 (`GameplayStatics.CreateSaveGameObject` "/Game/AdvWorldInteraction/Blueprints/MapComponents/ComponentsSaves/Save_Inventory.Save_Inventory_C"))
      (set `self.SaveGAme` _returnvalue_3)))
  (set `/Game/AdvWorldInteraction/Blueprints/MapComponents/ComponentsSaves/Save_Inventory.sInventory` (`self.Inventory`) (`self.SaveGAme`))
  (`GameplayStatics.SaveGameToSlot` (`self.SaveGAme`) (`self.InventorySlot`)))

(fn `UpdateInventory`
  (`/Engine/EditorBlueprintResources/StandardMacros.IsValid` (`self.Player`)
    (:`Is Valid`
      (`/Game/AdvWorldInteraction/UI/Widgets/Inventory/WB_Inventory.Update` (`self.Widget`)))))