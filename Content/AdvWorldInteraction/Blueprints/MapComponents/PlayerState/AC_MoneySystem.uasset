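; Player money component that tracks the owning actor's current balance and persists it between sessions.
; It loads the balance from a Save_Money slot on BeginPlay, and SaveMoney writes it back, creating the save object if none exists.
; AddMoney changes the balance and refreshes the experience and money widget through the owner's AC_MainWidgetHandler, but does not save.
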(event `self.ReceiveBeginPlay`
  (`self.LoadMoney`))

(fn `AddMoney`
  (params (Value :type "Float (double-precision)"))
  (bind _returnvalue (`Actor.GetComponentByClass` (`self.GetOwner`) "/Game/AdvWorldInteraction/Blueprints/WidgetHandler/AC_MainWidgetHandler.AC_MainWidgetHandler_C"))
  (bind _wb_maingui (`/Game/AdvWorldInteraction/Blueprints/WidgetHandler/AC_MainWidgetHandler.WB_MainGUI` _returnvalue))
  (bind _wb_expandmoney (`/Game/AdvWorldInteraction/UI/Widgets/Menu/WB_MainGUI.WB_ExpAndMoney` _wb_maingui))
  (set `self.CurrentMoney` (+ (`self.CurrentMoney`) Value))
  (`/Engine/EditorBlueprintResources/StandardMacros.IsValid` _returnvalue
    (:`Is Valid`
      (`/Engine/EditorBlueprintResources/StandardMacros.IsValid` _wb_maingui
        (:`Is Valid`
          (`/Engine/EditorBlueprintResources/StandardMacros.IsValid` _wb_expandmoney
            (:`Is Valid`
              (`/Game/AdvWorldInteraction/UI/Widgets/Player/WB_ExpAndMoney.UpdateVariables` _wb_expandmoney))))))))

(fn `LoadMoney`
  (bind _returnvalue (`GameplayStatics.DoesSaveGameExist` (`self.MoneySlot`)))
  (if _returnvalue
    (bind _returnvalue_2 (`GameplayStatics.LoadGameFromSlot` (`self.MoneySlot`)))
    (bind _assave_money (cast `/Game/AdvWorldInteraction/Blueprints/MapComponents/ComponentsSaves/Save_Money` _returnvalue_2))
    (set `self.CurrentMoney` (`/Game/AdvWorldInteraction/Blueprints/MapComponents/ComponentsSaves/Save_Money.sMoney` _assave_money))))

(fn `SaveMoney`
  (bind _returnvalue (`GameplayStatics.DoesSaveGameExist` (`self.MoneySlot`)))
  (if _returnvalue
    (bind _returnvalue_2 (`GameplayStatics.LoadGameFromSlot` (`self.MoneySlot`)))
    (bind _assave_money (cast `/Game/AdvWorldInteraction/Blueprints/MapComponents/ComponentsSaves/Save_Money` _returnvalue_2))
    (set `self.SaveGAme` _assave_money)
    (else
      (bind _returnvalue_3 (`GameplayStatics.CreateSaveGameObject` "/Game/AdvWorldInteraction/Blueprints/MapComponents/ComponentsSaves/Save_Money.Save_Money_C"))
      (set `self.SaveGAme` _returnvalue_3)))
  (set `/Game/AdvWorldInteraction/Blueprints/MapComponents/ComponentsSaves/Save_Money.sMoney` (`self.CurrentMoney`) (`self.SaveGAme`))
  (`GameplayStatics.SaveGameToSlot` (`self.SaveGAme`) (`self.MoneySlot`)))