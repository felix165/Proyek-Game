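; Actor component on the player character that plays a time speedup effect, shown from an overhead camera.
; SpeedupTime plays an optional sound, spawns a BP_TimeCamera high above the character, then blends to and possesses it.
; It raises global time dilation for a delay scaled by that dilation, then restores normal speed and blends back to re-possess the character.
; BeginPlay caches the owning character and its player controller.
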(event `self.ReceiveBeginPlay`
  ;[1 1 1] Initialize
  (bind _ascharacter (cast `Character` (`self.GetOwner`)))
  (set `self.MainCharacter` _ascharacter)
  (bind _asplayer_controller (cast `PlayerController` (`Pawn.GetController` _ascharacter)))
  (set `self.PlayerController` _asplayer_controller))

(event `SpeedupTime`
  (bind (_returnvalue_x _returnvalue_y _returnvalue_z) (`KismetMathLibrary.BreakVector` (`Actor.K2_GetActorLocation` (`self.GetOwner`))))
  ;[1 1 1] Start Speedup Time Effect
  (`self.TryPlayTimeSound`)
  (bind _returnvalue (`|SpawnActorFromClass` "/Game/AdvWorldInteraction/Blueprints/TimeManagment/BP_TimeCamera.BP_TimeCamera_C" (`KismetMathLibrary.MakeTransform` (`KismetMathLibrary.MakeVector` _returnvalue_x _returnvalue_y (+ _returnvalue_z 1000.0))) "Undefined" "OverrideRootScale" null null))
  (bind _output_get (set `self.NewPawn` _returnvalue))
  (`PlayerController.SetViewTargetWithBlend` (`self.PlayerController`) _output_get 1.0 "VTBlend_Linear" 0.0 false)
  (`KismetSystemLibrary.Delay` 0.8)
  (`Controller.Possess` (`self.PlayerController`) (`self.NewPawn`))
  (`GameplayStatics.SetGlobalTimeDilation` (`self.TimeDilation`))
  (`KismetSystemLibrary.Delay` (* (`self.TimeSpeedupDuration`) (/ (`self.TimeDilation`) 4.0)))
  (`GameplayStatics.SetGlobalTimeDilation` 1.0)
  (`PlayerController.SetViewTargetWithBlend` (`self.PlayerController`) (`self.MainCharacter`) 1.0 "VTBlend_Linear" 0.0 false)
  (`KismetSystemLibrary.Delay` 0.8)
  (`Controller.Possess` (`self.PlayerController`) (`self.MainCharacter`)))

(fn `TryPlayTimeSound`
  (bind _eventsound (`self.EventSound`))
  (`/Engine/EditorBlueprintResources/StandardMacros.IsValid` _eventsound
    (:`Is Valid`
      (`GameplayStatics.PlaySoundAtLocation` _eventsound (`Actor.K2_GetActorLocation` (`self.MainCharacter`))))))